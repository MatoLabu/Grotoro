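; BP_Title is the animated Grotoro title logo, which also serves as the countdown into gameplay.
; MoveUp and BackToCenter reposition and rescale the letter anchor.
; Counter flashes the GRO, TO and RO syllables on timed delays, then bounces the whole word, pairing each beat with a parameterized audio event and BP_PawnCamera shakes.
; It finally calls PhaseGame through GetPCont and removes itself with a short lifespan.
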(event Custom|MoveUp
  (bind _titleanchor (Variables|Default|GetTitleAnchor))
  (Transformation|SetRelativeLocation _titleanchor "0,-950.000000, 0" false false)
  (Variables|Default|SetSavedRelativeScale3D (Variables|/Script/Engine.SceneComponent|GetRelativeScale3D _titleanchor))
  (Transformation|SetRelativeScale3D _titleanchor "0.700000,0.700000,0.700000"))

(event Custom|BackToCenter
  (bind _titleanchor (Variables|Default|GetTitleAnchor))
  (Transformation|SetRelativeLocation _titleanchor "0, 0, 0" false false)
  (Transformation|SetRelativeScale3D _titleanchor (Variables|Default|GetSavedRelativeScale3D)))

(event Custom|Counter
  (bind _cameraref (Variables|Default|GetCameraREF))
  (Transformation|SetRelativeLocation (Variables|Default|GetTitleAnchor) "0,-500.000000, 0" false false)
  (Rendering|SetVisibility (Variables|Default|GetPlane) false false)
  (CallFunction|HideLetters)
  (Utilities|FlowControl|Delay 0.5)
  (Rendering|SetVisibility (Variables|Default|Get3O) true false)
  (CallFunction|SfxTitle 0.0)
  (Default|ShakeGro (Variables|Default|GetCameraREF))
  (Utilities|FlowControl|Delay 0.7)
  (CallFunction|HideLetters)
  (Utilities|FlowControl|Delay 0.1)
  (Rendering|SetVisibility (Variables|Default|Get4T) true false)
  (CallFunction|SfxTitle 1.0)
  (Default|ShakeGro (Variables|Default|GetCameraREF))
  (Utilities|FlowControl|Delay 0.7)
  (CallFunction|HideLetters)
  (Utilities|FlowControl|Delay 0.1)
  (Rendering|SetVisibility (Variables|Default|Get7O) true false)
  (CallFunction|SfxTitle 2.0)
  (Default|ShakeGro (Variables|Default|GetCameraREF))
  (Utilities|FlowControl|Delay 0.6)
  (CallFunction|HideLetters)
  (Utilities|FlowControl|Delay 0.2)
  (Transformation|SetRelativeScale3D (Variables|Default|GetTitleAnchor) "1.000000,1.000000,1.000000")
  (CallFunction|ShowLettersandBounce)
  (CallFunction|SfxTitle 3.0)
  (Default|ShakeGro _cameraref)
  (Default|ShakeGrotoro _cameraref)
  (Utilities|FlowControl|Delay 1.0)
  (CallFunction|HideLetters)
  (Default|PhaseGame (CallFunction|GetPCont))
  (Actor|SetLifeSpan 0.01))

(event EventBeginPlay
  ;[1 1 1] camera ref
  (bind _outactors (Actor|GetAllActorsOfClass "/Game/Grotoro/Gameplay/Character/BP_PawnCamera.BP_PawnCamera_C"))
  (Variables|Default|SetCameraREF (Utilities|Array|Get(acopy) _outactors)))

(fn ConstructionScript
  (Variables|Default|SetLetters (Utilities|Array|MakeArray (Variables|Default|Get3O) (Variables|Default|Get4T) (Variables|Default|Get5O) (Variables|Default|Get7O) (Variables|Default|Get1G) (Variables|Default|Get2R) (Variables|Default|Get6R))))

(fn HideLetters
  (for _array_element (Variables|Default|GetLetters)
    (Rendering|SetVisibility _array_element false false)))

(fn ShowLettersandBounce
  (for _array_element (Variables|Default|GetLetters)
    (Rendering|SetVisibility _array_element true false)
    (bind _asbp_letter (Utilities|Casting|CastToBP_Letter (Variables|/Script/Engine.ChildActorComponent|GetChildActor _array_element)))
    (Default|Bounce _asbp_letter)
    (Default|Bounce _asbp_letter)))

(fn SfxTitle
  (params (Parameter :type Float%20%28single-precision%29))
  (bind _returnvalue (Class|FMODBlueprintStatics|PlayEvent2D "/Game/FMOD/Events/SFx/A_Gameplay_BeginPlay.A_Gameplay_BeginPlay" false))
  (Class|FMODBlueprintStatics|EventInstanceSetParameter _returnvalue "BeginPlay" Parameter)
  (Class|FMODBlueprintStatics|EventInstancePlay _returnvalue))