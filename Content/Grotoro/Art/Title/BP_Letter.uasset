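; Animated 3D title letter (G, R, O or T, chosen in construction) that wobbles and shifts colour on the title screen.
; Looping timelines with random lengths and start times sample a shared oscillation curve to drive rotation, scale, Y offset and material colour every tick.
; Bounce plays an FMOD sound and adds clamped boosts to speed and amplitudes, which Tick eases back to rest at set speeds.
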(event Custom|Bounce
  ;[1 1 1] Bounce
  (Variables|Default|SetRate_Current (Math|Float|Clamp(Float) (+ (Variables|Default|GetRate_Current) (Variables|Default|GetRateBounceAddForce)) 1.0 3.0))
  (Variables|Default|SetBounceRotCoef (Math|Float|Clamp(Float) (+ (Variables|Default|GetBounceRotCoef) (Variables|Default|GetRotBounceAddForce)) 1.0 3.0))
  (Variables|Default|SetBounceScaleForceAdded (Math|Float|Clamp(Float) (+ (Variables|Default|GetBounceScaleForceAdded) (Variables|Default|GetScaleBounceAddForce)) 0.0 3.7))
  (Variables|Default|SetBounceColorMaxDif (Math|Float|Clamp(Float) (+ (Variables|Default|GetBounceColorMaxDif) (Variables|Default|GetColorMaxAddedValue))))
  (Variables|Default|SetBounceColorMinDif (Math|Float|Clamp(Float) (+ (Variables|Default|GetBounceColorMinDif) (Variables|Default|GetColorMinAddedValue))))
  (Variables|Default|SetBounceTransYForceAdded (Math|Float|Clamp(Float) (+ (Variables|Default|GetBounceTransYForceAdded) (Variables|Default|GetTransYAddedValue)) 0.0 7.5e+02))
  (Class|FMODAudioComponent|Play (Variables|Default|GetFMODAudio)))

(event EventBeginPlay
  (bind _returnvalue (Math|Random|RandomFloatinRange 0.25 0.5))
  (bind _r (Variables|Default|GetR))
  (bind _g (Variables|Default|GetG))
  (bind _b (Variables|Default|GetB))
  (bind _color_frequencymin (Variables|Default|GetColor_FrequencyMin))
  (bind _color_frequencymax (Variables|Default|GetColor_FrequencyMax))
  (bind _ty (Variables|Default|GetTY))
  (bind _rot_frequencymin (Variables|Default|GetRot_FrequencyMin))
  (bind _rot_frequencymax (Variables|Default|GetRot_FrequencyMax))
  (bind _scale_frequencymin (Variables|Default|GetScale_FrequencyMin))
  (bind _scale_frequencymax (Variables|Default|GetScale_FrequencyMax))
  (bind _y (Variables|Default|GetY))
  (bind _x (Variables|Default|GetX))
  (bind _sz (Variables|Default|GetSZ))
  (bind _z (Variables|Default|GetZ))
  (bind _sx (Variables|Default|GetSX))
  (bind _sy (Variables|Default|GetSY))
  (bind _returnvalue_2 (Math|Random|RandomFloatinRange _scale_frequencymin _scale_frequencymax))
  (bind _returnvalue_3 (Math|Random|RandomFloatinRange _scale_frequencymin _scale_frequencymax))
  (bind _returnvalue_4 (Math|Random|RandomFloatinRange _color_frequencymin _color_frequencymax))
  (bind _returnvalue_5 (Math|Random|RandomFloatinRange _color_frequencymin _color_frequencymax))
  (bind _returnvalue_6 (Math|Random|RandomFloatinRange _color_frequencymin _color_frequencymax))
  (bind _returnvalue_7 (Math|Random|RandomFloatinRange _scale_frequencymin _scale_frequencymax))
  (bind _returnvalue_8 (Math|Random|RandomFloatinRange _rot_frequencymin _rot_frequencymax))
  (bind _returnvalue_9 (Math|Random|RandomFloatinRange _rot_frequencymin _rot_frequencymax))
  (bind _returnvalue_10 (Math|Random|RandomFloatinRange _rot_frequencymin _rot_frequencymax))
  ;[0.07773 1 0] Begin Play
  (Utilities|FlowControl|Sequence
    (:then_0
      (bind _output_get (Variables|Default|SetFirstY _returnvalue_8))
      (CallFunction|RandomStartTime _y _output_get)
      (Timeline|Y Play
        (:Finished
          (Components|Timeline|SetTimelineLength _y _returnvalue_8)
          (Timeline|Y PlayFromStart))))
    (:then_1
      (bind _output_get_2 (Variables|Default|SetFirstX _returnvalue_9))
      (CallFunction|RandomStartTime _x _output_get_2)
      (Timeline|X Play
        (:Finished
          (Components|Timeline|SetTimelineLength _x _returnvalue_9)
          (Timeline|X PlayFromStart))))
    (:then_2
      (bind _output_get_3 (Variables|Default|SetFirstZ _returnvalue_10))
      (CallFunction|RandomStartTime _z _output_get_3)
      (Timeline|Z Play
        (:Finished
          (Components|Timeline|SetTimelineLength _z _returnvalue_10)
          (Timeline|Z PlayFromStart))))
    (:then_3
      (bind _output_get_4 (Variables|Default|SetFirstR _returnvalue_4))
      (CallFunction|RandomStartTime _r _output_get_4)
      (Timeline|R Play
        (:Finished
          (Components|Timeline|SetTimelineLength _r _returnvalue_4)
          (Timeline|R PlayFromStart))))
    (:then_4
      (bind _output_get_5 (Variables|Default|SetFirstG _returnvalue_5))
      (CallFunction|RandomStartTime _g _output_get_5)
      (Timeline|G Play
        (:Finished
          (Components|Timeline|SetTimelineLength _g _returnvalue_5)
          (Timeline|G PlayFromStart))))
    (:then_5
      (bind _output_get_6 (Variables|Default|SetFirstB _returnvalue_6))
      (CallFunction|RandomStartTime _b _output_get_6)
      (Timeline|B Play
        (:Finished
          (Components|Timeline|SetTimelineLength _b _returnvalue_6)
          (Timeline|B PlayFromStart))))
    (:then_6
      (bind _output_get_7 (Variables|Default|SetFirstSX _returnvalue_2))
      (CallFunction|RandomStartTime _sx _output_get_7)
      (Timeline|SX Play
        (:Finished
          (Components|Timeline|SetTimelineLength _sx _returnvalue_2)
          (Timeline|SX PlayFromStart))))
    (:then_7
      (bind _output_get_8 (Variables|Default|SetFirstSY _returnvalue_3))
      (CallFunction|RandomStartTime _sy _output_get_8)
      (Timeline|SY Play
        (:Finished
          (Components|Timeline|SetTimelineLength _sy _returnvalue_3)
          (Timeline|SY PlayFromStart))))
    (:then_8
      (bind _output_get_9 (Variables|Default|SetFirstSZ _returnvalue_7))
      (CallFunction|RandomStartTime _sz _output_get_9)
      (Timeline|SZ Play
        (:Finished
          (Components|Timeline|SetTimelineLength _sz _returnvalue_7)
          (Timeline|SZ PlayFromStart))))
    (:then_9
      (bind _output_get_10 (Variables|Default|SetFirstTY _returnvalue))
      (CallFunction|RandomStartTime _ty _output_get_10)
      (Timeline|TY Play
        (:Finished
          (Components|Timeline|SetTimelineLength _ty _returnvalue)
          (Timeline|TY PlayFromStart))))))

(event EventTick
  (params (DeltaSeconds :type Float%20%28single-precision%29))
  (bind _bouncetransyforceadded (Variables|Default|GetBounceTransYForceAdded))
  (bind _returnvalue (+ 12.0 _bouncetransyforceadded))
  ;[1 0.898 0] Event Tick
  (Transformation|SetRelativeRotation (Variables|Default|GetSM_Title_G1) (Math|Rotator|MakeRotator (CallFunction|RotbyCurve (Variables|Default|GetX) (Variables|Default|GetXForce)) (CallFunction|RotbyCurve (Variables|Default|GetY) (Variables|Default|GetYForce)) (CallFunction|RotbyCurve (Variables|Default|GetZ) (Variables|Default|GetZForce))) false false)
  (Rendering|Material|SetVectorParameterValue (Variables|Default|GetDynamicMat) "Color" (Math|Color|MakeColor (CallFunction|ColorinRangebyCurve (Variables|Default|GetR) 0.7 1.0) (CallFunction|ColorinRangebyCurve (Variables|Default|GetG) 0.05 0.4) (CallFunction|ColorinRangebyCurve (Variables|Default|GetB) 0.05 0.3)) :!class /Script/Engine.MaterialInstanceDynamic)
  (Transformation|SetRelativeScale3D (Variables|Default|GetSM_Title_G1) (Math|Vector|MakeVector (CallFunction|ScaleinRangebyCurve (Variables|Default|GetSX) 0.85 1.0) (CallFunction|ScaleinRangebyCurve (Variables|Default|GetSY) 0.85 1.0) (CallFunction|ScaleinRangebyCurve (Variables|Default|GetSZ) 0.1 0.5)))
  (Transformation|SetRelativeLocation (Variables|Default|GetSM_Title_G1) (Math|Vector|MakeVector 0.0 (- (* (Math|Curves|GetFloatValue (Variables|Default|GetCRV_Oscillation) (CallFunction|GetTimelinePercentage (Variables|Default|GetTY))) _returnvalue 2.0) _returnvalue) 0.0) false false)
  ;[1 1 1] Rate
  (CallFunction|SetAllRates (Variables|Default|GetRate_Current))
  (CallFunction|FadeRateto1))

(fn ConstructionScript
  (Components|StaticMesh|SetStaticMesh (Variables|Default|GetSM_Title_G1) (Utilities|Select :Index (Variables|Default|GetLetter) :Option%200 "/Game/Grotoro/Art/Title/SM_Title_G.SM_Title_G" :Option%201 "/Game/Grotoro/Art/Title/SM_Title_R.SM_Title_R" :Option%202 "/Game/Grotoro/Art/Title/SM_Title_O.SM_Title_O" :Option%203 "/Game/Grotoro/Art/Title/SM_Title_T.SM_Title_T"))
  (bind _returnvalue (Rendering|Material|CreateDynamicMaterialInstance (Variables|Default|GetSM_Title_G1) 0 "/Game/Grotoro/Art/Title/M_TitleLetter.M_TitleLetter" :!class /Script/Engine.PrimitiveComponent))
  (Variables|Default|SetDynamicMat _returnvalue))

(fn RotbyCurve
  (params (Timeline :type Timeline%20Component%20Object%20Reference) (Force :type Float%20%28single-precision%29))
  (bind _bouncerotcoef (Variables|Default|GetBounceRotCoef))
  (bind _returnvalue (* Force _bouncerotcoef))
  (return (- (* (Math|Curves|GetFloatValue (Variables|Default|GetCRV_Oscillation) (CallFunction|GetTimelinePercentage Timeline)) _returnvalue 2.0) _returnvalue)))

(fn ColorinRangebyCurve
  (params (Timeline :type Timeline%20Component%20Object%20Reference) (Min :type Float%20%28single-precision%29) (Max :type Float%20%28single-precision%29))
  (bind _bouncecolormindif (Variables|Default|GetBounceColorMinDif))
  (bind _returnvalue (- Min _bouncecolormindif))
  (bind _returnvalue_2 (Math|Float|Clamp(Float) _returnvalue))
  (return (+ (* (Math|Curves|GetFloatValue (Variables|Default|GetCRV_Oscillation) (CallFunction|GetTimelinePercentage Timeline)) (- (Math|Float|Clamp(Float) (+ Max (Variables|Default|GetBounceColorMaxDif))) _returnvalue_2)) _returnvalue_2)))

(fn SetAllRates
  (params (NewRate :type Float%20%28single-precision%29))
  (Components|Timeline|SetPlayRate (Variables|Default|GetY) NewRate))

(fn ScaleinRangebyCurve
  (params (Timeline :type Timeline%20Component%20Object%20Reference) (Min :type Float%20%28single-precision%29) (Max :type Float%20%28single-precision%29))
  (return (+ (* (Math|Curves|GetFloatValue (Variables|Default|GetCRV_Oscillation) (CallFunction|GetTimelinePercentage Timeline)) (- (+ Max (Variables|Default|GetBounceScaleForceAdded)) Min)) Min)))

(fn RandomStartTime
  (params (Timeline :type Timeline%20Component%20Object%20Reference) (Length :type Float%20%28single-precision%29))
  (Components|Timeline|SetTimelineLength Timeline Length)
  (Components|Timeline|SetNewTime Timeline (Math|Random|RandomFloatinRange 0.0 Length)))

(fn FadeRateto1
  (Utilities|FlowControl|Sequence
    (:then_0
      (if (> (Variables|Default|GetRate_Current) 1.0)
        (Variables|Default|SetRate_Current (select (< (- (Variables|Default|GetRate_Current) (* (Variables|Default|GetRateBackToNormalSpeed) (Utilities|Time|GetWorldDeltaSeconds))) 1.0) 1.0 (- (Variables|Default|GetRate_Current) (* (Variables|Default|GetRateBackToNormalSpeed) (Utilities|Time|GetWorldDeltaSeconds)))))))
    (:then_1
      (if (> (Variables|Default|GetBounceRotCoef) 1.0)
        (Variables|Default|SetBounceRotCoef (select (< (- (Variables|Default|GetBounceRotCoef) (* (Variables|Default|GetRotBackToNormalSpeed) (Utilities|Time|GetWorldDeltaSeconds))) 1.0) 1.0 (- (Variables|Default|GetBounceRotCoef) (* (Variables|Default|GetRotBackToNormalSpeed) (Utilities|Time|GetWorldDeltaSeconds)))))))
    (:then_2
      (if (> (Variables|Default|GetBounceScaleForceAdded) 0.0)
        (Variables|Default|SetBounceScaleForceAdded (select (< (- (Variables|Default|GetBounceScaleForceAdded) (* (Variables|Default|GetScaleBackToNormalSpeed) (Utilities|Time|GetWorldDeltaSeconds))) 0.0) 0.0 (- (Variables|Default|GetBounceScaleForceAdded) (* (Variables|Default|GetScaleBackToNormalSpeed) (Utilities|Time|GetWorldDeltaSeconds)))))))
    (:then_3
      (if (> (Variables|Default|GetBounceColorMaxDif) 0.0)
        (Variables|Default|SetBounceColorMaxDif (select (< (- (Variables|Default|GetBounceColorMaxDif) (* (Variables|Default|GetColorMaxBackToNormalSpeed) (Utilities|Time|GetWorldDeltaSeconds))) 0.0) 0.0 (- (Variables|Default|GetBounceColorMaxDif) (* (Variables|Default|GetColorMaxBackToNormalSpeed) (Utilities|Time|GetWorldDeltaSeconds)))))))
    (:then_4
      (if (> (Variables|Default|GetBounceColorMinDif) 0.0)
        (Variables|Default|SetBounceColorMinDif (select (< (- (Variables|Default|GetBounceColorMinDif) (* (Variables|Default|GetColorMinBackToNormalSpeed) (Utilities|Time|GetWorldDeltaSeconds))) 0.0) 0.0 (- (Variables|Default|GetBounceColorMinDif) (* (Variables|Default|GetColorMinBackToNormalSpeed) (Utilities|Time|GetWorldDeltaSeconds)))))))
    (:then_5
      (if (> (Variables|Default|GetBounceTransYForceAdded) 0.0)
        (Variables|Default|SetBounceTransYForceAdded (select (< (- (Variables|Default|GetBounceTransYForceAdded) (* (Variables|Default|GetTransYBackToNormalSpeed) (Utilities|Time|GetWorldDeltaSeconds))) 0.0) 0.0 (- (Variables|Default|GetBounceTransYForceAdded) (* (Variables|Default|GetTransYBackToNormalSpeed) (Utilities|Time|GetWorldDeltaSeconds)))))))))