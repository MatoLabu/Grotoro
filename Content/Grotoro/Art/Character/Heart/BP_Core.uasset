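; BP_Core is a pulsing core piece for the Heart character art, shown as a membrane, core or soft core.
; SetVisual uses MeshID to pick the mesh, material and scale range, with a narrower range for the membrane.
; Three timelines loop independently, taking a new random length on each pass.
; Tick samples an oscillation curve at each timeline's progress to scale X, Y and Z separately, giving an irregular organic wobble.
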(event Custom|SetVisual
  (bind _meshid (Variables|Default|GetMeshID))
  (Components|StaticMesh|SetStaticMesh (Variables|Default|GetCore) (Utilities|Select :Index _meshid :Option%200 "/Game/Grotoro/Art/Character/Heart/Membrane_mesh.Membrane_mesh" :Option%201 "/Game/Grotoro/Art/Character/Heart/Core_mesh.Core_mesh" :Option%202 "/Game/Grotoro/Art/Character/Heart/Core_soft_mesh.Core_soft_mesh"))
  (Rendering|Material|SetMaterial (Variables|Default|GetCore) 0 (Utilities|Select :Index _meshid :Option%200 "/Game/Grotoro/Art/Character/Heart/M_MembraneCore_Inst.M_MembraneCore_Inst" :Option%201 "/Game/Grotoro/Art/Character/Heart/M_MainFresnel_Core_Inst.M_MainFresnel_Core_Inst" :Option%202 "/Game/Grotoro/Art/Character/Heart/M_MainFresnel_Core_Inst.M_MainFresnel_Core_Inst"))
  (Variables|Default|SetScaleMin (Utilities|Select :Index _meshid :Option%200 0.95 :Option%201 0.7 :Option%202 0.7))
  (Variables|Default|SetScaleMax (Utilities|Select :Index _meshid :Option%200 1.05 :Option%201 1.3 :Option%202 1.3)))

(event EventTick
  (params (DeltaSeconds :type Float%20%28single-precision%29))
  (bind _scalemin (Variables|Default|GetScaleMin))
  (bind _scalemax (Variables|Default|GetScaleMax))
  (bind _scalemin_2 (Variables|Default|GetScaleMin))
  (bind _returnvalue (- _scalemax _scalemin_2))
  (Transformation|SetRelativeScale3D (Variables|Default|GetCore) (Math|Vector|MakeVector (+ _scalemin (* _returnvalue (Math|Curves|GetFloatValue (Variables|Default|GetCRV_Osc) (CallFunction|GetTimelinePercentage (Variables|Default|GetSX))))) (+ _scalemin (* _returnvalue (Math|Curves|GetFloatValue (Variables|Default|GetCRV_Osc) (CallFunction|GetTimelinePercentage (Variables|Default|GetSY))))) (+ _scalemin (* _returnvalue (Math|Curves|GetFloatValue (Variables|Default|GetCRV_Osc) (CallFunction|GetTimelinePercentage (Variables|Default|GetSZ))))))))

(event EventBeginPlay
  (Utilities|FlowControl|Sequence
    (:then_0
      (Components|Timeline|SetTimelineLength (Variables|Default|GetSX) (Math|Random|RandomFloatinRange 0.5 1.5) :!label _label)
      (Timeline|SX PlayFromStart
        (:Finished
          (goto _label))))
    (:then_1
      (Components|Timeline|SetTimelineLength (Variables|Default|GetSY) (Math|Random|RandomFloatinRange 0.5 1.5) :!label _label_2)
      (Timeline|SY PlayFromStart
        (:Finished
          (goto _label_2))))
    (:then_2
      (Components|Timeline|SetTimelineLength (Variables|Default|GetSZ) (Math|Random|RandomFloatinRange 0.5 1.5) :!label _label_3)
      (Timeline|SZ PlayFromStart
        (:Finished
          (goto _label_3))))))

(fn ConstructionScript)