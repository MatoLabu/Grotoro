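; BP_WallImpacts is a short-lived wall impact effect built from a flattened sphere mesh.
; The construction script randomizes the sphere's width and applies a dynamic material with exposed main and Fresnel colors plus random opacity and exponent.
; On BeginPlay a timeline with configurable length scales the sphere along one of five randomly chosen curves, sampled by playback percentage, then the actor expires when it finishes.
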(event EventBeginPlay
  (Variables|Default|SetCRV_Impact (Utilities|Select :Index (Math|Random|RandomIntegerinRange 0 4) :Option%200 "/Game/Grotoro/Art/Impacts/CRV_Impact01.CRV_Impact01" :Option%201 "/Game/Grotoro/Art/Impacts/CRV_Impact02.CRV_Impact02" :Option%202 "/Game/Grotoro/Art/Impacts/CRV_Impact03.CRV_Impact03" :Option%203 "/Game/Grotoro/Art/Impacts/CRV_Impact04.CRV_Impact04" :Option%204 "/Game/Grotoro/Art/Impacts/CRV_Impact05.CRV_Impact05"))
  (Components|Timeline|SetTimelineLength (Variables|Default|GetScaleAndLife) (Variables|Default|GetTimelineLenght))
  (Variables|Default|SetBaseScale (Variables|/Script/Engine.SceneComponent|GetRelativeScale3D (Variables|Default|GetSphere)))
  (Timeline|ScaleAndLife PlayFromStart
    (:Update
      (Transformation|SetRelativeScale3D (Variables|Default|GetSphere) (* (Variables|Default|GetBaseScale) (Math|Curves|GetFloatValue (Variables|Default|GetCRV_Impact) (CallFunction|GetTimelinePercentage (Variables|Default|GetScaleAndLife))))))
    (:Finished
      (Actor|SetLifeSpan 0.001))))

(fn ConstructionScript
  (bind _max_sphere_width (Variables|Default|GetMax%20Sphere%20Width))
  (bind _returnvalue (Math|Random|RandomFloatinRange 3.0 _max_sphere_width))
  (Transformation|SetRelativeScale3D (Variables|Default|GetSphere) (Math|Vector|MakeVector _returnvalue _returnvalue 0.1))
  (bind _returnvalue_2 (Rendering|Material|CreateDynamicMaterialInstance (Variables|Default|GetSphere) 0 "/Game/Grotoro/Art/Impacts/M_WallImpacts_Inst.M_WallImpacts_Inst" :!class /Script/Engine.PrimitiveComponent))
  (Rendering|Material|SetVectorParameterValue _returnvalue_2 "MainColor" (Variables|Default|GetWallImpactColor) :!class /Script/Engine.MaterialInstanceDynamic)
  (Rendering|Material|SetScalarParameterValue _returnvalue_2 "Opacity" (Math|Random|RandomFloatinRange 0.5 1.0) :!class /Script/Engine.MaterialInstanceDynamic)
  (Rendering|Material|SetScalarParameterValue _returnvalue_2 "ExponentIn" (Math|Random|RandomFloatinRange 0.5 1e+01) :!class /Script/Engine.MaterialInstanceDynamic)
  (Rendering|Material|SetVectorParameterValue _returnvalue_2 "FresnelColor" (Variables|Default|GetFresnelColor) :!class /Script/Engine.MaterialInstanceDynamic))