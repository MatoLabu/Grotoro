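; Single controller for Grotoro's two local players that drives the game phases from title through how-to-play, counter, game and game over.
; Each button's effect depends on the GameMode phase, while stick axes become eight-way headings that Tick feeds to each player's move.
; Timelines act as idle timeouts back to title or to a level restart.
; BeginPlay applies low scalability and lowers screen percentage if FPS is poor before starting.
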(event Custom|PhaseHowToPlay
  ;[1 1 1] Phase HowToPlay
  (Variables|/Game/Grotoro/Gameplay/BP_GameMode.BP_GameMode_C|SetPhase (CallFunction|GetGM) "NewEnumerator1")
  (Default|MoveUp (Variables|Default|GetBPTitleRef))
  (Default|LoadInstruction (Variables|Default|GetUITitleScreenRef))
  (Default|LaunchParticles (Variables|Default|GetBP_Ground))
  (Utilities|FlowControl|Sequence
    (:then_0
      (Timeline|DelayBeforeBackToTitle PlayFromStart
        (:Finished
          ;[1 1 1] usefull to not cut music
          (CallFunction|PhaseTitle)
          (Variables|Default|SetCanSkipHowToPlay false))))
    (:then_1
      (Utilities|FlowControl|Delay 0.3)
      (Variables|Default|SetCanSkipHowToPlay true))))

(event Custom|PhaseGame
  ;[1 1 1] Phase Game
  (Variables|/Game/Grotoro/Gameplay/BP_GameMode.BP_GameMode_C|SetPhase (CallFunction|GetGM) "NewEnumerator3")
  (Default|MusicState (Variables|Default|GetBp_SoundManager) 2.0 0.0)
  (Timeline|DelayBeforeRestartGame PlayFromStart
    (:Finished
      (Development|ExecuteConsoleCommand "restartlevel"))))

(event Custom|ResetDelayRestarGame
  (Timeline|DelayBeforeRestartGame PlayFromStart
    (:Finished
      (Development|ExecuteConsoleCommand "restartlevel"))))

(event Custom|PhaseTitle
  ;[1 1 1] Phase Title
  (Variables|/Game/Grotoro/Gameplay/BP_GameMode.BP_GameMode_C|SetPhase (CallFunction|GetGM) "NewEnumerator0")
  (Default|BacktoCenter (Variables|Default|GetBPTitleRef))
  (Default|HideInstructions (Variables|Default|GetUITitleScreenRef))
  (Default|MusicState (Variables|Default|GetBp_SoundManager) 1.0 0.0))

(event Custom|PhaseGameOver
  ;[1 1 1] Phase GameOver
  (Variables|/Game/Grotoro/Gameplay/BP_GameMode.BP_GameMode_C|SetPhase (CallFunction|GetGM) "NewEnumerator4")
  (Default|MusicState (Variables|Default|GetBp_SoundManager) 2.0 1.0)
  (Default|DeactivateParticles (Variables|Default|GetBP_Ground)))

(event Custom|PhaseCounter
  ;[1 1 1] Phase Counter
  (Utilities|FlowControl|Sequence
    (:then_0
      (Timeline|DelayBeforeBackToTitle Stop
        (:Finished
          ;[1 1 1] usefull to not cut music
          (CallFunction|PhaseTitle)
          (Variables|Default|SetCanSkipHowToPlay false))))
    (:then_1
      (Variables|/Game/Grotoro/Gameplay/BP_GameMode.BP_GameMode_C|SetPhase (CallFunction|GetGM) "NewEnumerator2")
      (Default|Counter (Variables|Default|GetBPTitleRef))
      (Rendering|SetActorHiddenInGame (Variables|Default|GetPlayer1) false)
      (Default|HideMainMenu (Variables|Default|GetUITitleScreenRef)))))

(event Custom|BounceTitleSound
  (bind _a_bouncesound (Variables|Default|GetA_BounceSound))
  (Class|FMODAudioComponent|SetParameter _a_bouncesound "BallsType" (Math|Conversions|ToFloat(Integer) (Math|Random|RandomIntegerinRange 0 3)))
  (Class|FMODAudioComponent|Play _a_bouncesound)
  ;[1 1 1] reset cooldown
  (Components|Timeline|SetPlaybackPosition (Variables|Default|GetDelayBeforeBackToTitle) 0.0 false true))

(event EventTick
  (params (DeltaSeconds :type Float%20%28single-precision%29))
  (bind _p1yvalue (Variables|Default|GetP1YValue))
  (bind _wanteddirection (Variables|Default|GetWantedDirection))
  (bind _p2xvalue (Variables|Default|GetP2XValue))
  (bind _p2yvalue (Variables|Default|GetP2YValue))
  (bind _p1xvalue (Variables|Default|GetP1XValue))
  ;[1 0.933 0] EVENT TICK
  (Variables|Default|SetFPS (/ 1.0 DeltaSeconds))
  (if (and (Utilities|IsValid (Variables|Default|GetPlayer1)) (Utilities|IsValid (Variables|Default|GetPlayer2)))
    (Utilities|FlowControl|Sequence
      (:then_0
        (if (or (!= _p1yvalue 0.0) (!= _p1xvalue 0.0))
          (CallFunction|PlayerGetWantedRotation _p1yvalue _p1xvalue)
          (Variables|Default|SetP1WantedDirection _wanteddirection)
          (Default|MoveandRotate (Variables|Default|GetPlayer1))))
      (:then_1
        (if (or (!= _p2yvalue 0.0) (!= _p2xvalue 0.0))
          (CallFunction|PlayerGetWantedRotation _p2yvalue _p2xvalue)
          (Variables|Default|SetP2WantedDirection _wanteddirection)
          (Default|MoveandRotate (Variables|Default|GetPlayer2)))))))

(event EventBeginPlay
  (bind _screenpercentage (Variables|Default|GetScreenPercentage))
  (bind _fps (Variables|Default|GetFPS))
  (bind _screenpercentage_2 (Variables|Default|GetScreenPercentage))
  (bind _returnvalue (Utilities|String|Append _screenpercentage "50"))
  (bind _returnvalue_2 (Utilities|String|Append _screenpercentage_2 "75"))
  ;[0.03288 1 0] BEGIN PLAY
  (Utilities|FlowControl|Sequence
    (:then_0
      (Utilities|FlowControl|Sequence
        (:then_0
          ;[1 1 1] Set Listenner Position
          (bind _outactors (Actor|GetAllActorsOfClass "/Game/Grotoro/Sound/Bp_SoundManager.Bp_SoundManager_C"))
          (bind _output_get (Variables|Default|SetBp_SoundManager (Utilities|Array|Get(acopy) _outactors)))
          (Class|PlayerController|SetAudioListenerOverride (Variables|/Game/Grotoro/Sound/Bp_SoundManager.Bp_SoundManager_C|GetListener _output_get) "0, 0, 0" "0, 0, 0")
          (bind _outactors_2 (Actor|GetAllActorsOfClass "/Game/Grotoro/Gameplay/LevelDesign/Bp_Ground.Bp_Ground_C"))
          (Variables|Default|SetBP_Ground (Utilities|Array|Get(acopy) _outactors_2))
          ;[1 1 1] Delay before skip title
          (Utilities|FlowControl|Delay 0.3)
          (Variables|Default|SetCanSkipTitle true))
        (:then_1
          (Utilities|FlowControl|Delay 0.2)
          (CallFunction|MakeTitleREF)
          (CallFunction|MakeUITitleScreenREF)
          (CallFunction|MakeCameraREF))))
    (:then_1
      ;[1 1 1] Scalability Settings
      (Development|PrintString "Set rendering parameters")
      (CallFunction|SetRendering)
      (Utilities|FlowControl|Delay 1.0)
      (Development|PrintString (Utilities|String|ToString(Float) _fps))
      (if (< _fps 55.0)
        (Development|PrintString _returnvalue_2)
        (Development|ExecuteConsoleCommand _returnvalue_2)
        (Utilities|FlowControl|Delay 2.0)
        (if (< (Variables|Default|GetFPS) 55.0)
          (Development|PrintString _returnvalue)
          (Development|ExecuteConsoleCommand _returnvalue)))
      (Variables|Default|SetGameIsReady true)
      (Default|StartGame (Variables|Default|GetBPTitleRef)))))

(event Input|ActionEvents|InputActionP1Olé
  (params (Key :type Key%20Structure))
  (:Pressed
    (switch Utilities|FlowControl|Switch|SwitchonE_GamePhase (Variables|/Game/Grotoro/Gameplay/BP_GameMode.BP_GameMode_C|GetPhase (CallFunction|GetGM))
      (:NewEnumerator0
        (if (and (Variables|Default|GetCanSkipTitle) (Variables|Default|GetGameIsReady))
          (CallFunction|PhaseHowtoPlay)))
      (:NewEnumerator1
        (if (Variables|Default|GetCanSkipHowToPlay)
          (CallFunction|PhaseCounter)))
      (:NewEnumerator3
        (Default|Ole (Variables|Default|GetPlayer1)))
      (:NewEnumerator4
        (if (Variables|/Game/Grotoro/Gameplay/BP_GameMode.BP_GameMode_C|GetCanRestart (CallFunction|GetGM))
          (Development|ExecuteConsoleCommand "restartlevel"))))))

(event Input|ActionEvents|InputActionP2Dash
  (params (Key :type Key%20Structure))
  (:Pressed
    (switch Utilities|FlowControl|Switch|SwitchonE_GamePhase (Variables|/Game/Grotoro/Gameplay/BP_GameMode.BP_GameMode_C|GetPhase (CallFunction|GetGM))
      (:NewEnumerator0
        (if (and (Variables|Default|GetCanSkipTitle) (Variables|Default|GetGameIsReady))
          (CallFunction|PhaseHowtoPlay)))
      (:NewEnumerator1
        (if (Variables|Default|GetCanSkipHowToPlay)
          (CallFunction|PhaseCounter)))
      (:NewEnumerator3
        (Default|Dash (Variables|Default|GetPlayer2)))
      (:NewEnumerator4
        (if (Variables|/Game/Grotoro/Gameplay/BP_GameMode.BP_GameMode_C|GetCanRestart (CallFunction|GetGM))
          (Development|ExecuteConsoleCommand "restartlevel"))))))

(event Input|ActionEvents|InputActionQuit
  (params (Key :type Key%20Structure))
  (:Pressed
    (Development|ExecuteConsoleCommand "EXIT")))

(event Input|ActionEvents|InputActionP2Olé
  (params (Key :type Key%20Structure))
  (:Pressed
    (switch Utilities|FlowControl|Switch|SwitchonE_GamePhase (Variables|/Game/Grotoro/Gameplay/BP_GameMode.BP_GameMode_C|GetPhase (CallFunction|GetGM))
      (:NewEnumerator0
        (if (and (Variables|Default|GetCanSkipTitle) (Variables|Default|GetGameIsReady))
          (CallFunction|PhaseHowtoPlay)))
      (:NewEnumerator1
        (if (Variables|Default|GetCanSkipHowToPlay)
          (CallFunction|PhaseCounter)))
      (:NewEnumerator3
        (Default|Ole (Variables|Default|GetPlayer2)))
      (:NewEnumerator4
        (if (Variables|/Game/Grotoro/Gameplay/BP_GameMode.BP_GameMode_C|GetCanRestart (CallFunction|GetGM))
          (Development|ExecuteConsoleCommand "restartlevel"))))))

(event Input|ActionEvents|InputActionDebugDirectStart
  (params (Key :type Key%20Structure)))

(event Input|ActionEvents|InputActionP1Dash
  (params (Key :type Key%20Structure))
  (:Pressed
    (switch Utilities|FlowControl|Switch|SwitchonE_GamePhase (Variables|/Game/Grotoro/Gameplay/BP_GameMode.BP_GameMode_C|GetPhase (CallFunction|GetGM))
      (:NewEnumerator0
        (if (and (Variables|Default|GetCanSkipTitle) (Variables|Default|GetGameIsReady))
          (CallFunction|PhaseHowtoPlay)))
      (:NewEnumerator1
        (if (Variables|Default|GetCanSkipHowToPlay)
          (CallFunction|PhaseCounter)))
      (:NewEnumerator3
        (Default|Dash (Variables|Default|GetPlayer1)))
      (:NewEnumerator4
        (if (Variables|/Game/Grotoro/Gameplay/BP_GameMode.BP_GameMode_C|GetCanRestart (CallFunction|GetGM))
          (Development|ExecuteConsoleCommand "restartlevel"))))))

(event Input|ActionEvents|InputActionTempRestart
  (params (Key :type Key%20Structure)))

(event Input|AxisEvents|InputAxisP1Y
  (params (AxisValue :type Float%20%28single-precision%29))
  (switch Utilities|FlowControl|Switch|SwitchonE_GamePhase (Variables|/Game/Grotoro/Gameplay/BP_GameMode.BP_GameMode_C|GetPhase (CallFunction|GetGM))
    (:NewEnumerator3
      _)
    (:NewEnumerator4
      _))
  (Variables|Default|SetP1YValue AxisValue))

(event Input|AxisEvents|InputAxisP1X
  (params (AxisValue :type Float%20%28single-precision%29))
  (switch Utilities|FlowControl|Switch|SwitchonE_GamePhase (Variables|/Game/Grotoro/Gameplay/BP_GameMode.BP_GameMode_C|GetPhase (CallFunction|GetGM))
    (:NewEnumerator3
      _)
    (:NewEnumerator4
      _))
  (Variables|Default|SetP1XValue AxisValue))

(event Input|AxisEvents|InputAxisP2Y
  (params (AxisValue :type Float%20%28single-precision%29))
  (switch Utilities|FlowControl|Switch|SwitchonE_GamePhase (Variables|/Game/Grotoro/Gameplay/BP_GameMode.BP_GameMode_C|GetPhase (CallFunction|GetGM))
    (:NewEnumerator3
      _)
    (:NewEnumerator4
      _))
  (Variables|Default|SetP2YValue AxisValue))

(event Input|AxisEvents|InputAxisP2X
  (params (AxisValue :type Float%20%28single-precision%29))
  (switch Utilities|FlowControl|Switch|SwitchonE_GamePhase (Variables|/Game/Grotoro/Gameplay/BP_GameMode.BP_GameMode_C|GetPhase (CallFunction|GetGM))
    (:NewEnumerator3
      _)
    (:NewEnumerator4
      _))
  (Variables|Default|SetP2XValue AxisValue))

(event Input|KeyboardEvents|V
  (params (Key :type Key%20Structure))
  ;[1 1 1] DEBUG
)

(event Input|KeyboardEvents|C
  (params (Key :type Key%20Structure))
  ;[1 1 1] DEBUG
)

(event Input|KeyboardEvents|AnyKey
  (params (Key :type Key%20Structure))
  (bind _gm (CallFunction|GetGM))
  (bind _gm_2 (CallFunction|GetGM))
  (bind _a_bouncesound (Variables|Default|GetA_BounceSound))
  (bind _phase (Variables|/Game/Grotoro/Gameplay/BP_GameMode.BP_GameMode_C|GetPhase _gm_2))
  (bind _phase_2 (Variables|/Game/Grotoro/Gameplay/BP_GameMode.BP_GameMode_C|GetPhase _gm))
  (:Pressed
    ;[1 1 1] Bounce title letters
    (if (or (Utilities|Enum|Equal(Enum) _phase_2 "NewEnumerator0") (Utilities|Enum|Equal(Enum) _phase_2 "NewEnumerator1"))
      (bind _outactors (Actor|GetAllActorsOfClass "/Game/Grotoro/Art/Title/BP_Letter.BP_Letter_C"))
      (for _array_element _outactors
        (if (not (Variables|/Game/Grotoro/Art/Title/BP_Letter.BP_Letter_C|GetIsBull _array_element))
          (Default|Bounce _array_element)))
      (Class|FMODAudioComponent|SetParameter _a_bouncesound "BallsType" (Math|Conversions|ToFloat(Integer) (Math|Random|RandomIntegerinRange 0 3)))
      (Class|FMODAudioComponent|Play _a_bouncesound)
      ;[1 1 1] reset cooldown
      (Components|Timeline|SetPlaybackPosition (Variables|Default|GetDelayBeforeBackToTitle) 0.0 false true)
      (elif (or (Utilities|Enum|Equal(Enum) _phase "NewEnumerator3") (Utilities|Enum|Equal(Enum) _phase "NewEnumerator4"))
        (CallFunction|ResetDelayRestarGame)))))

(event Input|KeyboardEvents|F
  (params (Key :type Key%20Structure))
  (:Pressed
    (Development|ExecuteConsoleCommand "stat unitgraph")
    (Development|ExecuteConsoleCommand "stat fps")))

(event Input|KeyboardEvents|G
  (params (Key :type Key%20Structure)))

(fn ConstructionScript)

(fn PlayerGetWantedRotation
  (params (PlayerYValue :type Float%20%28single-precision%29) (PlayerXValue :type Float%20%28single-precision%29))
  (if (and (== PlayerYValue 1.0) (== PlayerXValue 0.0))
    (Variables|Default|SetWantedDirection "0, 0, 0")
    (elif (and (== PlayerYValue -1.0) (== PlayerXValue 0.0))
      (Variables|Default|SetWantedDirection "0,180.000000, 0")
      (elif (and (== PlayerYValue 0.0) (== PlayerXValue 1.0))
        (Variables|Default|SetWantedDirection "0,90.000000, 0")
        (elif (and (== PlayerYValue 0.0) (== PlayerXValue -1.0))
          (Variables|Default|SetWantedDirection "0,270.000000, 0")
          (elif (and (== PlayerYValue 1.0) (== PlayerXValue 1.0))
            (Variables|Default|SetWantedDirection "0,45.000000, 0")
            (elif (and (== PlayerYValue -1.0) (== PlayerXValue 1.0))
              (Variables|Default|SetWantedDirection "0,135.000000, 0")
              (elif (and (== PlayerYValue 1.0) (== PlayerXValue -1.0))
                (Variables|Default|SetWantedDirection "0,315.000000, 0")
                (elif (and (== PlayerYValue -1.0) (== PlayerXValue -1.0))
                  (Variables|Default|SetWantedDirection "0,225.000000, 0"))))))))))

(fn HideTitle
  (Rendering|SetActorHiddenInGame (Variables|Default|GetBPTitleRef) true))

(fn MakeTitleREF
  (bind _outactors (Actor|GetAllActorsOfClass "/Game/Grotoro/Art/Title/BP_Title.BP_Title_C"))
  (bind _asbp_title (Utilities|Casting|CastToBP_Title (Utilities|Array|Get(acopy) _outactors)))
  (Variables|Default|SetBPTitleRef _asbp_title))

(fn MakeUITitleScreenREF
  (bind _foundwidgets (Widget|GetAllWidgetsOfClass "/Game/Grotoro/UI/UI_TitleScreen.UI_TitleScreen_C" true))
  (bind _asui_title_screen (Utilities|Casting|CastToUI_TitleScreen (Utilities|Array|Get(acopy) _foundwidgets)))
  (Variables|Default|SetUITitleScreenRef _asui_title_screen))

(fn MakeCameraREF
  (bind _outactors (Actor|GetAllActorsOfClass "/Game/Grotoro/Gameplay/Character/BP_PawnCamera.BP_PawnCamera_C"))
  (Variables|Default|SetREF_Camera (Utilities|Array|Get(acopy) _outactors)))

(fn SetRendering
  (Development|ExecuteConsoleCommand "r.vsynceditor 0")
  (Development|ExecuteConsoleCommand "r.vsync 0")
  (Development|ExecuteConsoleCommand "r.ViewDistanceScale 1")
  (Development|ExecuteConsoleCommand "r.PostProcessAAQuality 0")
  (Development|ExecuteConsoleCommand "sg.PostProcessQuality 0")
  (Development|ExecuteConsoleCommand "sg.ShadowQuality 0")
  (Development|ExecuteConsoleCommand "sg.TextureQuality 0")
  (Development|ExecuteConsoleCommand "sg.EffectsQuality 0")
  (Development|ExecuteConsoleCommand "r.DetailMode 0")
  (Development|ExecuteConsoleCommand "FoliageQuality 0"))

(fn SetScreenRes)