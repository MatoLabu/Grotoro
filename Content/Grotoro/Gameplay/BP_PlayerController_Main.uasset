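; Main player controller for Grotoro that drives both players and handles global keys, with Escape quitting.
; Each tick, non-zero axis values for each player become one of eight directions through exact-value matching, then that player moves and rotates.
; Depending on game phase, any key bounces title letters with a random sound and resets the back-to-title delay, or resets the restart delay.
; Helpers cache title, UI and camera references and apply low-quality rendering settings.
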(event Custom|BounceTitleSound
  (bind _a_bouncesound (Variables|Default|GetA_BounceSound))
  (Class|FMODAudioComponent|SetParameter _a_bouncesound "BallsType" (Math|Conversions|ToFloat(Integer) (Math|Random|RandomIntegerinRange 0 3)))
  (Class|FMODAudioComponent|Play _a_bouncesound)
  ;[1 1 1] reset cooldown
  (Components|Timeline|SetPlaybackPosition (Variables|/Game/Grotoro/Gameplay/BP_GameMode.BP_GameMode_C|GetDelayBeforeBackToTitle (CallFunction|GetGM)) 0.0 false true))

(event EventTick
  (params (DeltaSeconds :type Float%20%28single-precision%29))
  (bind _p1yvalue (Variables|Default|GetP1YValue))
  (bind _wanteddirection (Variables|Default|GetWantedDirection))
  (bind _p2xvalue (Variables|Default|GetP2XValue))
  (bind _p2yvalue (Variables|Default|GetP2YValue))
  (bind _p1xvalue (Variables|Default|GetP1XValue))
  ;[1 0.933 0] EVENT TICK
  (if (and (Utilities|IsValid (Variables|Default|GetPlayer1)) (Utilities|IsValid (Variables|Default|GetPlayer2)))
    (Utilities|FlowControl|Sequence
      (:then_0
        (if (or (!= _p1yvalue 0.0) (!= _p1xvalue 0.0))
          (CallFunction|PlayerGetWantedRotation _p1yvalue _p1xvalue)
          (Variables|Default|SetP1WantedDirection _wanteddirection)
          (Default|MoveandRotate (Variables|Default|GetPlayer1))))
      (:then_1
        (if (or (!= _p2yvalue 0.0) (!= _p2xvalue 0.0))
          (CallFunction|PlayerGetWantedRotation _p2yvalue _p2xvalue)
          (Variables|Default|SetP2WantedDirection _wanteddirection)
          (Default|MoveandRotate (Variables|Default|GetPlayer2)))))))

(event Input|KeyboardEvents|V
  (params (Key :type Key%20Structure))
  ;[1 1 1] DEBUG
)

(event Input|KeyboardEvents|C
  (params (Key :type Key%20Structure))
  ;[1 1 1] DEBUG
)

(event Input|KeyboardEvents|AnyKey
  (params (Key :type Key%20Structure))
  (bind _gm (CallFunction|GetGM))
  (bind _gm_2 (CallFunction|GetGM))
  (bind _a_bouncesound (Variables|Default|GetA_BounceSound))
  (bind _phase (Variables|/Game/Grotoro/Gameplay/BP_GameMode.BP_GameMode_C|GetPhase _gm_2))
  (bind _phase_2 (Variables|/Game/Grotoro/Gameplay/BP_GameMode.BP_GameMode_C|GetPhase _gm))
  (:Pressed
    ;[1 1 1] Bounce title letters
    (if (or (Utilities|Enum|Equal(Enum) _phase_2 "NewEnumerator0") (Utilities|Enum|Equal(Enum) _phase_2 "NewEnumerator1"))
      (bind _outactors (Actor|GetAllActorsOfClass "/Game/Grotoro/Art/Title/BP_Letter.BP_Letter_C"))
      (for _array_element _outactors
        (if (not (Variables|/Game/Grotoro/Art/Title/BP_Letter.BP_Letter_C|GetIsBull _array_element))
          (Default|Bounce _array_element)))
      (Class|FMODAudioComponent|SetParameter _a_bouncesound "BallsType" (Math|Conversions|ToFloat(Integer) (Math|Random|RandomIntegerinRange 0 3)))
      (Class|FMODAudioComponent|Play _a_bouncesound)
      ;[1 1 1] reset cooldown
      (Components|Timeline|SetPlaybackPosition (Variables|/Game/Grotoro/Gameplay/BP_GameMode.BP_GameMode_C|GetDelayBeforeBackToTitle (CallFunction|GetGM)) 0.0 false true)
      (elif (or (Utilities|Enum|Equal(Enum) _phase "NewEnumerator3") (Utilities|Enum|Equal(Enum) _phase "NewEnumerator4"))
        (Default|ResetDelayRestarGame (CallFunction|GetGM))))))

(event Input|KeyboardEvents|F
  (params (Key :type Key%20Structure)))

(event Input|KeyboardEvents|G
  (params (Key :type Key%20Structure)))

(event Input|KeyboardEvents|Escape
  (params (Key :type Key%20Structure))
  (:Pressed
    (Development|ExecuteConsoleCommand "EXIT")))

(fn ConstructionScript)

(fn PlayerGetWantedRotation
  (params (PlayerYValue :type Float%20%28single-precision%29) (PlayerXValue :type Float%20%28single-precision%29))
  (if (and (== PlayerYValue 1.0) (== PlayerXValue 0.0))
    (Variables|Default|SetWantedDirection "0, 0, 0")
    (elif (and (== PlayerYValue -1.0) (== PlayerXValue 0.0))
      (Variables|Default|SetWantedDirection "0,180.000000, 0")
      (elif (and (== PlayerYValue 0.0) (== PlayerXValue 1.0))
        (Variables|Default|SetWantedDirection "0,90.000000, 0")
        (elif (and (== PlayerYValue 0.0) (== PlayerXValue -1.0))
          (Variables|Default|SetWantedDirection "0,270.000000, 0")
          (elif (and (== PlayerYValue 1.0) (== PlayerXValue 1.0))
            (Variables|Default|SetWantedDirection "0,45.000000, 0")
            (elif (and (== PlayerYValue -1.0) (== PlayerXValue 1.0))
              (Variables|Default|SetWantedDirection "0,135.000000, 0")
              (elif (and (== PlayerYValue 1.0) (== PlayerXValue -1.0))
                (Variables|Default|SetWantedDirection "0,315.000000, 0")
                (elif (and (== PlayerYValue -1.0) (== PlayerXValue -1.0))
                  (Variables|Default|SetWantedDirection "0,225.000000, 0"))))))))))

(fn HideTitle
  (Rendering|SetActorHiddenInGame (Variables|Default|GetBPTitleRef) true))

(fn MakeTitleREF
  (bind _outactors (Actor|GetAllActorsOfClass "/Game/Grotoro/Art/Title/BP_Title.BP_Title_C"))
  (Variables|Default|SetBPTitleRef (Utilities|Array|Get(acopy) _outactors)))

(fn MakeUITitleScreenREF
  (bind _foundwidgets (Widget|GetAllWidgetsOfClass "/Game/Grotoro/UI/UI_TitleScreen.UI_TitleScreen_C" true))
  (Variables|Default|SetUITitleScreenRef (Utilities|Array|Get(acopy) _foundwidgets)))

(fn MakeCameraREF
  (bind _outactors (Actor|GetAllActorsOfClass "/Game/Grotoro/Gameplay/Character/BP_PawnCamera.BP_PawnCamera_C"))
  (Variables|Default|SetREF_Camera (Utilities|Array|Get(acopy) _outactors)))

(fn SetRendering
  (bind _asbp_game_instance (CallFunction|GetGI))
  (if (Variables|/Game/Grotoro/Gameplay/BP_GameInstance.BP_GameInstance_C|GetFirstStart _asbp_game_instance)
    (Development|ExecuteConsoleCommand "r.ScreenPercentage 100")
    (Variables|/Game/Grotoro/Gameplay/BP_GameInstance.BP_GameInstance_C|SetFirstStart _asbp_game_instance false))
  (Development|ExecuteConsoleCommand "r.vsynceditor 0")
  (Development|ExecuteConsoleCommand "r.vsync 0")
  (Development|ExecuteConsoleCommand "r.ViewDistanceScale 1")
  (Development|ExecuteConsoleCommand "r.PostProcessAAQuality 4")
  (Development|ExecuteConsoleCommand "sg.PostProcessQuality 0")
  (Development|ExecuteConsoleCommand "sg.ShadowQuality 0")
  (Development|ExecuteConsoleCommand "sg.TextureQuality 0")
  (Development|ExecuteConsoleCommand "sg.EffectsQuality 0")
  (Development|ExecuteConsoleCommand "r.DetailMode 0")
  (Development|ExecuteConsoleCommand "FoliageQuality 0"))

(fn SetScreenRes)