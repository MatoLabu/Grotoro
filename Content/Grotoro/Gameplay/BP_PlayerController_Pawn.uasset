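; Two-player controller for Grotoro that routes attack and dodge input to each pawn's Dash and Ole, with Escape exiting the game.
; The game mode's Phase gates these buttons, so in Game Over they restart the level once CanRestart is set.
; P1 direction keys set axis values, with a Timeline driving Up, while P2's axis logic is disconnected.
; Helper functions, uncalled here, map axes to eight-way rotation, cache title and camera references, and apply low-quality rendering settings.
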(event EventTick
  (params (DeltaSeconds :type Float%20%28single-precision%29))
  ;[1 0.933 0] EVENT TICK
)

(event EventBeginPlay
  ;[0.03288 1 0] BEGIN PLAY
)

(event Input|ActionEvents|InputActionP1Attack
  (params (Key :type Key%20Structure))
  (:Pressed
    (switch Utilities|FlowControl|Switch|SwitchonE_GamePhase (Variables|/Game/Grotoro/Gameplay/BP_GameMode.BP_GameMode_C|GetPhase (CallFunction|GetGM))
      (:NewEnumerator3
        (Default|Dash (Variables|Default|GetPlayer1)))
      (:NewEnumerator4
        (if (Variables|/Game/Grotoro/Gameplay/BP_GameMode.BP_GameMode_C|GetCanRestart (CallFunction|GetGM))
          (Development|ExecuteConsoleCommand "restartlevel"))))))

(event Input|ActionEvents|InputActionP2Attack
  (params (Key :type Key%20Structure))
  (:Pressed
    (switch Utilities|FlowControl|Switch|SwitchonE_GamePhase (Variables|/Game/Grotoro/Gameplay/BP_GameMode.BP_GameMode_C|GetPhase (CallFunction|GetGM))
      (:NewEnumerator3
        (Default|Dash (Variables|Default|GetPlayer2)))
      (:NewEnumerator4
        (if (Variables|/Game/Grotoro/Gameplay/BP_GameMode.BP_GameMode_C|GetCanRestart (CallFunction|GetGM))
          (Development|ExecuteConsoleCommand "restartlevel"))))))

(event Input|ActionEvents|InputActionP2Dodge
  (params (Key :type Key%20Structure))
  (:Pressed
    (switch Utilities|FlowControl|Switch|SwitchonE_GamePhase (Variables|/Game/Grotoro/Gameplay/BP_GameMode.BP_GameMode_C|GetPhase (CallFunction|GetGM))
      (:NewEnumerator3
        (Default|Ole (Variables|Default|GetPlayer2)))
      (:NewEnumerator4
        (if (Variables|/Game/Grotoro/Gameplay/BP_GameMode.BP_GameMode_C|GetCanRestart (CallFunction|GetGM))
          (Development|ExecuteConsoleCommand "restartlevel"))))))

(event Input|ActionEvents|InputActionP1Up
  (params (Key :type Key%20Structure))
  (:Pressed
    (Timeline|Timeline_0 PlayFromStart
      (:Update
        (Variables|Default|SetP1Up true)
        (switch Utilities|FlowControl|Switch|SwitchonE_GamePhase (Variables|/Game/Grotoro/Gameplay/BP_GameMode.BP_GameMode_C|GetPhase (CallFunction|GetGM))
          (:NewEnumerator3
            _)
          (:NewEnumerator4
            _))
        (Variables|Default|SetP1YValue (select (Variables|Default|GetP1Up) 1.0 -1.0)))))
  (:Released
    (Timeline|Timeline_0 Stop)))

(event Input|ActionEvents|InputActionP1Down
  (params (Key :type Key%20Structure))
  (:Pressed
    (Variables|Default|SetP1Up false)
    (switch Utilities|FlowControl|Switch|SwitchonE_GamePhase (Variables|/Game/Grotoro/Gameplay/BP_GameMode.BP_GameMode_C|GetPhase (CallFunction|GetGM))
      (:NewEnumerator3
        _)
      (:NewEnumerator4
        _))
    (Variables|Default|SetP1YValue (select (Variables|Default|GetP1Up) 1.0 -1.0))))

(event Input|ActionEvents|InputActionP1Left
  (params (Key :type Key%20Structure))
  (:Pressed
    (Variables|Default|SetP1Left true)
    (switch Utilities|FlowControl|Switch|SwitchonE_GamePhase (Variables|/Game/Grotoro/Gameplay/BP_GameMode.BP_GameMode_C|GetPhase (CallFunction|GetGM)) :!label _label
      (:NewEnumerator3
        _)
      (:NewEnumerator4
        _))
    (Variables|Default|SetP1XValue (select (Variables|Default|GetP1Right) 1.0 -1.0)))
  (:Released
    (Variables|Default|SetP1Left false)
    (goto _label)))

(event Input|ActionEvents|InputActionP1Right
  (params (Key :type Key%20Structure))
  (:Pressed
    (Variables|Default|SetP1Right true)
    (switch Utilities|FlowControl|Switch|SwitchonE_GamePhase (Variables|/Game/Grotoro/Gameplay/BP_GameMode.BP_GameMode_C|GetPhase (CallFunction|GetGM)) :!label _label
      (:NewEnumerator3
        _)
      (:NewEnumerator4
        _))
    (Variables|Default|SetP1XValue (select (Variables|Default|GetP1Right) 1.0 -1.0)))
  (:Released
    (Variables|Default|SetP1Right false)
    (goto _label)))

(event Input|ActionEvents|InputActionP1Dodge
  (params (Key :type Key%20Structure))
  (:Pressed
    (switch Utilities|FlowControl|Switch|SwitchonE_GamePhase (Variables|/Game/Grotoro/Gameplay/BP_GameMode.BP_GameMode_C|GetPhase (CallFunction|GetGM))
      (:NewEnumerator3
        (Default|Ole (Variables|Default|GetPlayer1)))
      (:NewEnumerator4
        (if (Variables|/Game/Grotoro/Gameplay/BP_GameMode.BP_GameMode_C|GetCanRestart (CallFunction|GetGM))
          (Development|ExecuteConsoleCommand "restartlevel"))))))

(event Input|KeyboardEvents|Escape
  (params (Key :type Key%20Structure))
  (:Pressed
    (Development|ExecuteConsoleCommand "EXIT")))

(fn ConstructionScript)

(fn PlayerGetWantedRotation
  (params (PlayerYValue :type Float%20%28single-precision%29) (PlayerXValue :type Float%20%28single-precision%29))
  (if (and (== PlayerYValue 1.0) (== PlayerXValue 0.0))
    (Variables|Default|SetWantedDirection "0, 0, 0")
    (elif (and (== PlayerYValue -1.0) (== PlayerXValue 0.0))
      (Variables|Default|SetWantedDirection "0,180.000000, 0")
      (elif (and (== PlayerYValue 0.0) (== PlayerXValue 1.0))
        (Variables|Default|SetWantedDirection "0,90.000000, 0")
        (elif (and (== PlayerYValue 0.0) (== PlayerXValue -1.0))
          (Variables|Default|SetWantedDirection "0,270.000000, 0")
          (elif (and (== PlayerYValue 1.0) (== PlayerXValue 1.0))
            (Variables|Default|SetWantedDirection "0,45.000000, 0")
            (elif (and (== PlayerYValue -1.0) (== PlayerXValue 1.0))
              (Variables|Default|SetWantedDirection "0,135.000000, 0")
              (elif (and (== PlayerYValue 1.0) (== PlayerXValue -1.0))
                (Variables|Default|SetWantedDirection "0,315.000000, 0")
                (elif (and (== PlayerYValue -1.0) (== PlayerXValue -1.0))
                  (Variables|Default|SetWantedDirection "0,225.000000, 0"))))))))))

(fn HideTitle
  (Rendering|SetActorHiddenInGame (Variables|Default|GetBPTitleRef) true))

(fn MakeTitleREF
  (bind _outactors (Actor|GetAllActorsOfClass "/Game/Grotoro/Art/Title/BP_Title.BP_Title_C"))
  (Variables|Default|SetBPTitleRef (Utilities|Array|Get(acopy) _outactors)))

(fn MakeUITitleScreenREF
  (bind _foundwidgets (Widget|GetAllWidgetsOfClass "/Game/Grotoro/UI/UI_TitleScreen.UI_TitleScreen_C" true))
  (Variables|Default|SetUITitleScreenRef (Utilities|Array|Get(acopy) _foundwidgets)))

(fn MakeCameraREF
  (bind _outactors (Actor|GetAllActorsOfClass "/Game/Grotoro/Gameplay/Character/BP_PawnCamera.BP_PawnCamera_C"))
  (Variables|Default|SetREF_Camera (Utilities|Array|Get(acopy) _outactors)))

(fn SetRendering
  (bind _asbp_game_instance (CallFunction|GetGI))
  (if (Variables|/Game/Grotoro/Gameplay/BP_GameInstance.BP_GameInstance_C|GetFirstStart _asbp_game_instance)
    (Development|ExecuteConsoleCommand "r.ScreenPercentage 100")
    (Variables|/Game/Grotoro/Gameplay/BP_GameInstance.BP_GameInstance_C|SetFirstStart _asbp_game_instance false))
  (Development|ExecuteConsoleCommand "r.vsynceditor 0")
  (Development|ExecuteConsoleCommand "r.vsync 0")
  (Development|ExecuteConsoleCommand "r.ViewDistanceScale 1")
  (Development|ExecuteConsoleCommand "r.PostProcessAAQuality 4")
  (Development|ExecuteConsoleCommand "sg.PostProcessQuality 0")
  (Development|ExecuteConsoleCommand "sg.ShadowQuality 0")
  (Development|ExecuteConsoleCommand "sg.TextureQuality 0")
  (Development|ExecuteConsoleCommand "sg.EffectsQuality 0")
  (Development|ExecuteConsoleCommand "r.DetailMode 0")
  (Development|ExecuteConsoleCommand "FoliageQuality 0"))

(fn SetScreenRes)