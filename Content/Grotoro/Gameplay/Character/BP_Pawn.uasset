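; Player pawn for a two-player bull duel, where dash hits cost life and shed a fat ball, and a hit at zero life ends the game.
; A physics ball rolls by torque with the body snapped onto it; Life drives fat scale and, through curves, move and turn speed.
; Overlaps resolve bounces, hits and dash clashes, while timelines run Dash, the Olé jump-dodge and hurt blinking, with camera and sound feedback.
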(event OnComponentBeginOverlap(TriggerSphere)
  (params (OverlappedComponent :type Primitive%20Component%20Object%20Reference) (OtherActor :type Actor%20Object%20Reference) (OtherComp :type Primitive%20Component%20Object%20Reference) (OtherBodyIndex :type Integer) (bFromSweep :type Boolean) (SweepResult :type Hit%20Result%20Structure%20%28by%20ref%29))
  (bind _bodyanchor (Variables|Default|GetBodyAnchor))
  (bind _rivalpawn_ref (Variables|Default|GetRivalPawn_REF))
  ;[1 1 1] Collision
  ;[1 1 1] TOUCH OTHER PLAYER
  (if (Components|ComponentHasTag OtherComp "fat")
    (CallFunction|HitMaterial)
    (CallFunction|MakeRefOfOtherPlayer)
    (bind _returnvalue (Physics|GetPhysicsLinearVelocity (Variables|Default|GetBall) "None"))
    (Variables|Default|SetMyBounceVelocity (Math|Vector|NegateVector (Math|Vector|MakeVector (.x _returnvalue) (.y _returnvalue) 0.0)))
    (if (and (not (Variables|Default|GetIsDashing)) (not (Variables|BP_Pawn_C|GetIsDashing (Variables|Default|GetRivalPawn_REF))))
      ;[1 1 1] Bounce
      (bind _returnvalue_2 (Physics|GetPhysicsLinearVelocity (Variables|BP_Pawn_C|GetBall (Variables|Default|GetRivalPawn_REF)) "None"))
      (Variables|Default|SetBounceDirection (* (Math|Vector|Normalize (- (Transformation|GetWorldLocation (Variables|Default|GetBall)) (Transformation|GetWorldLocation (Variables|BP_Pawn_C|GetBall (Variables|Default|GetRivalPawn_REF))))) (select (>= (Math|Vector|VectorLength (Variables|Default|GetMyBounceVelocity)) (Math|Vector|VectorLength _returnvalue_2)) (Math|Vector|VectorLength (Variables|Default|GetMyBounceVelocity)) (Math|Vector|VectorLength _returnvalue_2))))
      (Physics|SetPhysicsLinearVelocity (Variables|Default|GetBall) (Variables|Default|GetBounceDirection) false "None")
      (elif (Math|Boolean|ANDBoolean (Variables|Default|GetIsDashing) (not (Variables|BP_Pawn_C|GetIsDashing _rivalpawn_ref)) (not (Variables|BP_Pawn_C|GetIsHurt _rivalpawn_ref)) (not (Variables|BP_Pawn_C|GetIsDodging _rivalpawn_ref)))
        (Class|FMODAudioComponent|Play (Variables|Default|GetA_Hit))
        (CallFunction|HitMe (Variables|Default|GetRivalPawn_REF))
        (CallFunction|StopDash)
        (elif (and (Variables|Default|GetIsDashing) (Variables|BP_Pawn_C|GetIsDashing (Variables|Default|GetRivalPawn_REF)))
          (CallFunction|StopDash)
          (Class|FMODAudioComponent|Play (Variables|Default|GetA_Block))
          ;[1 1 1] CS
          (Default|CSDashVsDash (Variables|Default|GetREF_Camera))
          ;[1 1 1] Double Bounce
          (Default|Bounce (Variables|Default|GetBullBodyREF))
          (Default|Bounce (Variables|Default|GetBullBodyREF)))))
    (else
      (bind _asbp_wall_collision (Utilities|Casting|CastToBP_WallCollision OtherActor))
      (Variables|Default|SetCollidedWall _asbp_wall_collision)
      (if (Variables|Default|GetIsDashing)
        (Transformation|SetWorldRotation (Variables|/Game/Grotoro/Gameplay/LevelDesign/BP_WallCollision.BP_WallCollision_C|GetPawnDirection (Variables|Default|GetCollidedWall)) (Transformation|GetWorldRotation _bodyanchor) false false)
        (Transformation|SetRelativeRotation (Variables|/Game/Grotoro/Gameplay/LevelDesign/BP_WallCollision.BP_WallCollision_C|GetBouncePawnDirection (Variables|Default|GetCollidedWall)) (Variables|/Script/Engine.SceneComponent|GetRelativeRotation (Variables|/Game/Grotoro/Gameplay/LevelDesign/BP_WallCollision.BP_WallCollision_C|GetPawnDirection (Variables|Default|GetCollidedWall))) false false)
        (Transformation|SetWorldRotation _bodyanchor (Math|Rotator|MakeRotator 0.0 0.0 (.yaw (Transformation|GetWorldRotation (Variables|/Game/Grotoro/Gameplay/LevelDesign/BP_WallCollision.BP_WallCollision_C|GetBouncePawnDirection (Variables|Default|GetCollidedWall))))) false false)
        ;[1 1 1] CS
        (Default|CSDashinWall (Variables|Default|GetREF_Camera))))))

(event Custom|Dash
  (if (Math|Boolean|ANDBoolean (Variables|Default|GetDashEnable) (not (Variables|Default|GetIsGlue)) (not (Variables|Default|GetIsDodging)))
    (Variables|Default|SetIsDashing true)
    (Variables|Default|SetDashEnable false)
    (Development|SetHiddeninGame (Variables|Default|GetDashFX) false false)
    ;[1 1 1] CS
    (Default|CSDMidAMidFLow (Variables|Default|GetREF_Camera))
    ;[1 1 1] Dash bounce
    (Default|Bounce (Variables|Default|GetBullBodyREF))
    (Class|FMODAudioComponent|Play (Variables|Default|GetA_Dash))
    (Development|SetHiddeninGame (Variables|Default|GetYaaa%20!) false true)
    (Utilities|FlowControl|Sequence
      (:then_0
        (Components|Timeline|SetTimelineLength (Variables|Default|GetT_DashDuration) (Variables|Default|GetDashDuration))
        (Timeline|T_DashDuration PlayFromStart
          (:Update
            (Physics|SetPhysicsLinearVelocity (Variables|Default|GetBall) (* (Math|Vector|GetForwardVector (Variables|Default|GetDirection)) 2e+03) false "None"))
          (:Finished
            (Development|SetHiddeninGame (Variables|Default|GetDashFX) true false)
            (Utilities|FlowControl|Delay 0.01)
            (Variables|Default|SetIsDashing false))))
      (:then_1
        (Components|Timeline|SetTimelineLength (Variables|Default|GetT_DashCooldown) (Variables|Default|GetDashCooldown))
        (Timeline|T_DashCooldown PlayFromStart
          (:Finished
            (Variables|Default|SetDashEnable true)
            (Development|SetHiddeninGame (Variables|Default|GetYaaa%20!) true true)))))))

(event Custom|HitMaterial
  (bind _m_bouncing (Variables|Default|GetM_Bouncing))
  ;[1 1 1] HIT MATERIAL
  (bind _scalar (Timeline|GlueScale PlayFromStart)
    (:Update
      (Rendering|Material|SetScalarParameterValue _m_bouncing "Multiplier" (* _scalar 3e+01) :!class /Script/Engine.MaterialInstanceDynamic)
      (Rendering|Material|SetScalarParameterValue _m_bouncing "Speed" 2.0 :!class /Script/Engine.MaterialInstanceDynamic))
    (:Finished
      (Rendering|Material|SetScalarParameterValue _m_bouncing "Speed" 1.0 :!class /Script/Engine.MaterialInstanceDynamic))))

(event Custom|Ole
  (bind _ball (Variables|Default|GetBall))
  (bind _ball_2 (Variables|Default|GetBall))
  (bind _returnvalue (Transformation|GetWorldLocation _ball_2))
  (if (and (not (Variables|Default|GetIsDashing)) (not (Variables|Default|GetIsOleing)))
    (Variables|Default|SetIsOleing true)
    (Variables|Default|SetIsDodging true)
    (Utilities|FlowControl|Sequence
      (:then_0
        (Development|SetHiddeninGame (Variables|Default|GetOlé) false true)
        (Collision|SetCollisionResponsetoChannel (Variables|Default|GetBall) "ECC_PhysicsBody" "ECR_Ignore")
        ;[1 1 1] CS
        (Default|CSOleJump (Variables|Default|GetREF_Camera))
        ;[1 1 1] sfx
        (Class|FMODAudioComponent|Play (Variables|Default|GetA_Ole))
        (Physics|SetSimulatePhysics (Variables|Default|GetBall) false)
        (Variables|Default|SetOleBodyAnchorStartRot (Variables|/Script/Engine.SceneComponent|GetRelativeRotation (Variables|Default|GetBodyAnchor)))
        (Variables|Default|SetRandomSideOleRotation (select (Math|Random|RandomBool) -1.0 1.0)))
      (:then_1
        (Utilities|FlowControl|Sequence
          (:then_0
            (Components|Timeline|SetTimelineLength (Variables|Default|GetT_DodgeCooldown) 0.75)
            (Timeline|T_DodgeCooldown PlayFromStart
              (:Update
                (Transformation|SetWorldLocation _ball_2 (Math|Vector|MakeVector (.x _returnvalue) (.y _returnvalue) (* (Math|Curves|GetFloatValue (Variables|Default|GetCRV_OleJump) (CallFunction|GetTimelinePercentage (Variables|Default|GetT_DodgeCooldown))) 8e+03)) false false)
                (Transformation|SetRelativeRotation (Variables|Default|GetBodyAnchor) (Math|Rotator|MakeRotator (.roll (Variables|Default|GetOleBodyAnchorStartRot)) (.pitch (Variables|Default|GetOleBodyAnchorStartRot)) (+ (.yaw (Variables|Default|GetOleBodyAnchorStartRot)) (* (Math|Curves|GetFloatValue (Variables|Default|GetCRV_OleRotation) (CallFunction|GetTimelinePercentage (Variables|Default|GetT_DodgeCooldown))) 3.6e+02 2.0 (Variables|Default|GetRandomSideOleRotation)))) false false))
              (:Finished
                (Variables|Default|SetIsDodging false)
                (Collision|SetCollisionResponsetoChannel (Variables|Default|GetBall) "ECC_PhysicsBody" "ECR_Block")
                (Transformation|SetRelativeRotation (Variables|Default|GetBodyAnchor) (Variables|Default|GetOleBodyAnchorStartRot) false false)
                (Physics|SetPhysicsLinearVelocity _ball "0, 0, 0" false "None")
                (Physics|SetSimulatePhysics _ball true)
                ;[1 1 1] CS
                (Default|CSOleFall (Variables|Default|GetREF_Camera)))))
          (:then_2
            (Components|Timeline|SetTimelineLength (Variables|Default|GetT_OleCooldown) 1.25)
            (Timeline|T_OleCooldown PlayFromStart
              (:Finished
                (Variables|Default|SetIsOleing false)
                (Development|SetHiddeninGame (Variables|Default|GetOlé) true true)))))))))

(event Custom|StopDash
  (Utilities|FlowControl|Sequence
    (:then_0
      (Timeline|T_DashDuration Stop
        (:Update
          (Physics|SetPhysicsLinearVelocity (Variables|Default|GetBall) (* (Math|Vector|GetForwardVector (Variables|Default|GetDirection)) 2e+03) false "None"))
        (:Finished
          (Development|SetHiddeninGame (Variables|Default|GetDashFX) true false :!label _label)
          (Utilities|FlowControl|Delay 0.01)
          (Variables|Default|SetIsDashing false))))
    (:then_1
      (goto _label))))

(event Custom|MoveAndRotate
  (bind _pcont (CallFunction|GetPCont))
  (bind _targetdirection (Variables|Default|GetTargetDirection))
  (bind _dleft (Variables|Default|GetDLeft))
  (bind _targetdirection_2 (Variables|Default|GetTargetDirection))
  (bind _dright (Variables|Default|GetDRight))
  (bind _ball (Variables|Default|GetBall))
  (bind _returnvalue (Transformation|GetWorldLocation _dleft))
  (bind _returnvalue_2 (Transformation|GetWorldLocation _targetdirection_2))
  (bind _returnvalue_3 (Transformation|GetWorldLocation _dright))
  (bind _returnvalue_4 (Transformation|GetWorldLocation _targetdirection))
  (bind _returnvalue_5 (- _returnvalue_4 _returnvalue))
  (bind _returnvalue_6 (- _returnvalue_2 _returnvalue_3))
  (bind _returnvalue_7 (Math|Vector|VectorLength _returnvalue_6))
  (bind _returnvalue_8 (Math|Vector|VectorLength _returnvalue_5))
  (if (not (Variables|Default|GetIsDashing))
    (bind _output_get (Variables|Default|SetWantedRotation (Utilities|Select :Index (Variables|Default|GetPlayerID) :Option%200 "0, 0, 0" :Option%201 (Variables|/Game/Grotoro/Gameplay/BP_PlayerController.BP_PlayerController_C|GetP1WantedDirection _pcont) :Option%202 (Variables|/Game/Grotoro/Gameplay/BP_PlayerController.BP_PlayerController_C|GetP2WantedDirection _pcont))))
    (Transformation|SetWorldRotation (Variables|Default|GetWantedDirection) _output_get false false)
    (Utilities|FlowControl|Sequence
      (:then_0
        ;[1 1 1] secu for not shaking
        (if (or (> _returnvalue_8 1e+01) (> _returnvalue_7 1e+01))
          (Transformation|AddLocalRotation (Variables|Default|GetBodyAnchor) (Math|Rotator|MakeRotator 0.0 0.0 (* (select (>= _returnvalue_8 _returnvalue_7) 1.0 -1.0) (Utilities|Time|GetWorldDeltaSeconds) (Math|Curves|GetFloatValue (Variables|Default|GetCRV_RotSpeedByLife) (/ (Variables|Default|GetLife) 1e+02)))) false false)))
      (:then_1
        ;[1 1 1] Rolling (moving)
        (if (not (Variables|Default|GetIsGlue))
          (if (Physics|IsSimulatingPhysics _ball "None")
            (Class|PrimitiveComponent|AddTorqueinRadians _ball (* (Math|Vector|GetRightVector (Variables|Default|GetWantedDirection)) (* (Utilities|Time|GetWorldDeltaSeconds) (Math|Curves|GetFloatValue (Variables|Default|GetCRV_MoveSpeedByLife) (/ (Variables|Default|GetLife) 1e+02)) 1e+08)) "None" false)))))))

(event Custom|HitMe
  (bind _bodyanchor (Variables|Default|GetBodyAnchor))
  (bind _returnvalue (Transformation|GetWorldTransform _bodyanchor))
  ;[1 1 1] secu doublon
  (if (not (Variables|Default|GetIsHurt))
    (Variables|Default|SetIsHurt true)
    (if (== (Variables|Default|GetLife) 0.0)
      ;[1 1 1] DEATH
      (Actor|SetLifeSpan 0.001)
      (Default|PhaseGameOver (CallFunction|GetPCont))
      ;[1 1 1] CS
      (Default|CSDeath (Variables|Default|GetREF_Camera))
      (Default|GameOver (CallFunction|GetGM) (select (== (Variables|Default|GetPlayerID) 1) 2 1))
      (else
        (bind _newlife (CallFunction|LooseLife))
        ;[1 1 1] CS
        (Default|CSHit (Variables|Default|GetREF_Camera))
        ;[1 1 1] Hit Bounce
        (Default|Bounce (Variables|Default|GetBullBodyREF))
        (Default|Bounce (Variables|Default|GetBullBodyREF))
        (Default|LooseLife (Variables|Default|GetBpSoundManager) (Variables|Default|GetLife))
        (Utilities|FlowControl|Sequence
          (:then_0
            ;[1 1 1] 1PV
            (if (<= _newlife 0.0)
              (Default|BullHideBody (Variables|Default|GetBullBodyREF))
              ;[1 1 1] CS
              (Default|CS1PV (Variables|Default|GetREF_Camera))
              ;[1 1 1] sfx
              (bind _returnvalue_2 (Class|FMODBlueprintStatics|PlayEvent2D "/Game/FMOD/Events/SFx/A_1PVLeft.A_1PVLeft"))
              (Class|FMODBlueprintStatics|EventInstanceSetParameter _returnvalue_2 "PlayerPV" (Math|Conversions|ToFloat(Integer) (- (Variables|Default|GetPlayerID) 1)))))
          (:then_1
            ;[1 1 1] SPAWN FAT BALL
            (Game|SpawnActorfromClass "/Game/Grotoro/Gameplay/FatBall/BP_FatBall2.BP_FatBall2_C" (Math|Transform|MakeTransform (.location _returnvalue) (.rotation _returnvalue) "0.500000,0.500000,0.500000") "Undefined" 0 (Variables|Default|GetPlayerID) (Variables|Default|GetPlayerColor) (Variables|Default|GetSecondColor) 0)
            (Components|Timeline|SetTimelineLength (Variables|Default|GetT_HurtCooldown) 1.0)
            (Timeline|T_HurtCooldown PlayFromStart
              (:Update
                ;[1 1 1] Blink red
                (Variables|Default|SetPlayerColor (select (== (Math|Curves|GetFloatValue (Variables|Default|GetCRV_HurtBlinkRed) (Components|Timeline|GetPlaybackPosition (Variables|Default|GetT_HurtCooldown))) 1.0) "(R=1.000000,G=0.000000,B=0.000000,A=1.000000)" (Variables|Default|GetINITPlayerColor)))
                (Default|SetPlayerIdandColor (Variables|Default|GetBullBodyREF) (Variables|Default|GetPlayerID) (Variables|Default|GetPlayerColor) (Variables|Default|GetSecondColor)))
              (:Finished
                (Variables|Default|SetIsHurt false)
                (Variables|Default|SetPlayerColor (Variables|Default|GetINITPlayerColor))
                (Default|SetPlayerIdandColor (Variables|Default|GetBullBodyREF) (Variables|Default|GetPlayerID) (Variables|Default|GetPlayerColor) (Variables|Default|GetSecondColor))))))))))

(event EventTick
  (params (DeltaSeconds :type Float%20%28single-precision%29))
  ;[1 0.8934 0] EVENT TICK
  (CallFunction|SnapBodyonCore)
  ;[1 1 1] Set Fat Scale
  (CallFunction|SetFatScale)
  (CallFunction|SetBubbleLocationandRotation -1.7e+02 (Variables|Default|GetOlé))
  (CallFunction|SetBubbleLocationandRotation 1.7e+02 (Variables|Default|GetYaaa%20!))
  (CallFunction|SFXMove))

(event EventBeginPlay
  ;[0 1 0.03866] BEGIN PLAY
  (CallFunction|MoveSound)
  ;[1 1 1] secu INIT fat material
  (Variables|Default|SetFatMaterial (Variables|Default|GetFatMaterial_INIT))
  (bind _returnvalue (Rendering|Material|CreateDynamicMaterialInstance (Variables|Default|GetFat) 0 "/Game/Grotoro/Gameplay/Character/M_SimpleTrans_Inst_CharFat.M_SimpleTrans_Inst_CharFat" :!class /Script/Engine.PrimitiveComponent))
  (Variables|Default|SetM_Bouncing _returnvalue)
  (Utilities|FlowControl|Delay 0.2)
  (CallFunction|REFSoundManager)
  (CallFunction|REFCamera)
  (CallFunction|MakePlayerColor (Variables|Default|GetPlayerID))
  ;[1 1 1] Make Bull Body ref (BP_Letter)
  (bind _output_get (Variables|Default|SetBullBodyREF (.AsBP%20Letter (Utilities|Casting|CastToBP_Letter (Variables|/Script/Engine.ChildActorComponent|GetChildActor (Variables|Default|GetBP_Letter))))))
  (Default|SetPlayerIdandColor _output_get (Variables|Default|GetPlayerID) (Variables|Default|GetPlayerColor) (Variables|Default|GetSecondColor)))

(event Custom|Move%20Sound
  (bind _a_move (Variables|Default|GetA_Move))
  ;[1 1 1] >Play Move Sound
  (bind _returnvalue (Class|FMODAudioComponent|IsPlaying _a_move))
  (if (not _returnvalue)
    (Class|FMODAudioComponent|Play _a_move)
    (Class|FMODAudioComponent|SetParameter (Variables|Default|GetA_Move) "Moving" 0.0)))

(fn ConstructionScript
  (CallFunction|SetFatScale)
  (CallFunction|SnapBodyonCore)
  (Default|SetIsBull (.AsBP%20Letter (Utilities|Casting|CastToBP_Letter (Variables|/Script/Engine.ChildActorComponent|GetChildActor (Variables|Default|GetBP_Letter))))))

(fn SetFatScale
  (bind _life (Variables|Default|GetLife))
  (bind _returnvalue (/ _life 1e+02))
  (bind _returnvalue_2 (* _returnvalue 2.0))
  (bind _returnvalue_3 (+ _returnvalue_2 1.5))
  (if (> _life 0.0)
    (Transformation|SetRelativeScale3D (Variables|Default|GetFatAnchor) (Math|Vector|MakeVector _returnvalue_3 _returnvalue_3 _returnvalue_3))
    (else
      (Transformation|SetRelativeScale3D (Variables|Default|GetFatAnchor) (Math|Vector|MakeVector 1.0 1.0 1.0)))))

(fn SnapBodyonCore
  (bind _ball (Variables|Default|GetBall))
  (bind _returnvalue (Transformation|GetWorldLocation _ball))
  (Transformation|SetWorldLocation (Variables|Default|GetBodyAnchor) (Math|Vector|MakeVector (.x _returnvalue) (.y _returnvalue) (.z _returnvalue)) false false))

(fn MakeRefOfOtherPlayer
  (Utilities|IsValid (Variables|Default|GetRivalPawn_REF)
    (:Is%20Not%20Valid
      (bind _outactors (Actor|GetAllActorsOfClass "BP_Pawn_C"))
      (for _array_element _outactors
        (if (!= (Variables|BP_Pawn_C|GetPlayerID _array_element) (Variables|Default|GetPlayerID))
          (bind _asbp_pawn (Utilities|Casting|CastToBP_Pawn _array_element))
          (Variables|Default|SetRivalPawn_REF _asbp_pawn))))))

(fn SFXMove
  (bind _a_move (Variables|Default|GetA_Move))
  (if (Utilities|Enum|Equal(Enum) (Variables|/Game/Grotoro/Gameplay/BP_GameMode.BP_GameMode_C|GetPhase (CallFunction|GetGM)) "NewEnumerator3")
    (bind _returnvalue (Physics|GetPhysicsLinearVelocity (Variables|Default|GetBall) "None"))
    (Class|FMODAudioComponent|SetParameter (Variables|Default|GetA_Move) "Speed" (Math|Float|MapRangeClamped (Math|Vector|VectorLength (Math|Vector|MakeVector (.x _returnvalue) (.y _returnvalue) 0.0)) 1.5e+02 3e+03 0.0 1.0))
    (if (>= (Math|Vector|VectorLength (Math|Vector|MakeVector (.x _returnvalue) (.y _returnvalue) 0.0)) 5e+01)
      (Class|FMODAudioComponent|SetParameter _a_move "Moving" 1.0)
      (else
        (Class|FMODAudioComponent|SetParameter _a_move "Moving" 0.0)))))

(fn ResetFatMaterial
  (Rendering|Material|SetMaterial (Variables|Default|GetFat) 0 (Variables|Default|GetFatMaterial)))

(fn AskFatBalltoEjectMe
  (for _array_element (Collision|GetOverlappingActors (Variables|Default|GetTriggerSphere) "/Game/Grotoro/Gameplay/FatBall/BP_FatBall.BP_FatBall_C" :!class /Script/Engine.PrimitiveComponent)
    (bind _asbp_fat_ball (Utilities|Casting|CastToBP_FatBall _array_element))
    (Default|EjectPlayer _asbp_fat_ball)))

(fn SetBubbleLocationandRotation
  (params (Y :type Float%20%28single-precision%29) (BubbleText :type Text%20Render%20Component%20Object%20Reference))
  (bind _ball (Variables|Default|GetBall))
  (bind _returnvalue (Transformation|GetWorldLocation _ball))
  (Transformation|SetWorldRotation BubbleText "90.000000,180.000000,0.000000" false false)
  (Transformation|SetWorldLocation BubbleText (Math|Vector|MakeVector (+ (.x _returnvalue) Y) (.y _returnvalue) (+ (.z _returnvalue) 4.9e+02)) false false))

(fn REFSoundManager
  (bind _outactors (Actor|GetAllActorsOfClass "/Game/Grotoro/Sound/Bp_SoundManager.Bp_SoundManager_C"))
  (Utilities|IsValid (Utilities|Array|Get(acopy) _outactors)
    (:Is%20Valid
      (Variables|Default|SetBpSoundManager (Utilities|Array|Get(acopy) _outactors)))))

(fn REFCamera
  (bind _outactors (Actor|GetAllActorsOfClass "/Game/Grotoro/Gameplay/Character/BP_PawnCamera.BP_PawnCamera_C"))
  (Utilities|IsValid (Utilities|Array|Get(acopy) _outactors)
    (:Is%20Valid
      (Variables|Default|SetREF_Camera (Utilities|Array|Get(acopy) _outactors)))))

(fn LooseLife
  (bind _output_get (Variables|Default|SetLife (Math|Float|Clamp(Float) (- (Variables|Default|GetLife) 1e+01) 0.0 1e+02)))
  (return _output_get))

(fn MakePlayerColor
  (params (PlayerID :type Integer))
  (bind _returnvalue (- PlayerID 1))
  (bind _output_get (Variables|Default|SetPlayerColor (Utilities|Select :Index _returnvalue :Option%200 (Math|Color|MakeColor 0.0 0.1 0.0) :Option%201 (Math|Color|MakeColor 0.0 0.0 0.1))))
  (Variables|Default|SetINITPlayerColor _output_get)
  (Variables|Default|SetSecondColor (Utilities|Select :Index _returnvalue :Option%200 (Math|Color|MakeColor 0.0 1.0 1.0) :Option%201 (Math|Color|MakeColor 0.0 0.3 1.0)))
  (bind _asbp_heart (Utilities|Casting|CastToBP_Heart (Variables|/Script/Engine.ChildActorComponent|GetChildActor (Variables|Default|GetBP_Heart))))
  (Default|MakeColor _asbp_heart (Variables|Default|GetPlayerColor) (Variables|Default|GetSecondColor)))