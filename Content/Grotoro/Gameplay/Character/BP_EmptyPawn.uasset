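; BP_EmptyPawn is an input-only pawn that relays menu input during the title, how-to-play and game-over phases.
; Attack, dodge and left click advance the GM (likely game mode) on Title Screen or Game Over; on How to Play, only attack and dodge act, validating the pad player in UI_TitleScreen.
; Left/right go to that widget without phase checks, while any-key and quit inputs call GM actions directly.
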(event Input|ActionEvents|InputActionPadAttack
  (params (Key :type Key%20Structure))
  (bind _gm (CallFunction|GetGM))
  (:Pressed
    (switch Utilities|FlowControl|Switch|SwitchonE_GamePhase (Variables|/Game/Grotoro/Gameplay/BP_GameMode.BP_GameMode_C|GetPhase _gm)
      (:NewEnumerator0
        (Default|Next _gm :!label _label))
      (:NewEnumerator1
        (bind _foundwidgets (Widget|GetAllWidgetsOfClass "/Game/Grotoro/UI/UI_TitleScreen.UI_TitleScreen_C" true))
        (Default|PadPlayerValidation (Utilities|Array|Get(acopy) _foundwidgets)))
      (:NewEnumerator4
        (goto _label)))))

(event Input|ActionEvents|InputActionPadLeft
  (params (Key :type Key%20Structure))
  (:Pressed
    (bind _foundwidgets (Widget|GetAllWidgetsOfClass "/Game/Grotoro/UI/UI_TitleScreen.UI_TitleScreen_C" true))
    (Default|InputLeft (Utilities|Array|Get(acopy) _foundwidgets))))

(event Input|ActionEvents|InputActionPadDodge
  (params (Key :type Key%20Structure))
  (:Pressed
    (switch Utilities|FlowControl|Switch|SwitchonE_GamePhase (Variables|/Game/Grotoro/Gameplay/BP_GameMode.BP_GameMode_C|GetPhase (CallFunction|GetGM))
      (:NewEnumerator0
        (Default|Next (CallFunction|GetGM) :!label _label))
      (:NewEnumerator1
        (bind _foundwidgets (Widget|GetAllWidgetsOfClass "/Game/Grotoro/UI/UI_TitleScreen.UI_TitleScreen_C" true))
        (Default|PadPlayerValidation (Utilities|Array|Get(acopy) _foundwidgets)))
      (:NewEnumerator4
        (goto _label)))))

(event Input|ActionEvents|InputActionPadRight
  (params (Key :type Key%20Structure))
  (:Pressed
    (bind _foundwidgets (Widget|GetAllWidgetsOfClass "/Game/Grotoro/UI/UI_TitleScreen.UI_TitleScreen_C" true))
    (Default|InputRight (Utilities|Array|Get(acopy) _foundwidgets))))

(event Input|ActionEvents|InputActionPadQuit
  (params (Key :type Key%20Structure))
  (:Pressed
    (Default|ActionQuit (CallFunction|GetGM))))

(event Input|KeyboardEvents|AnyKey
  (params (Key :type Key%20Structure))
  (:Pressed
    (Default|AnyKeyActions (CallFunction|GetGM))))

(event Input|KeyboardEvents|Escape
  (params (Key :type Key%20Structure))
  (:Pressed
    (Default|ActionQuit (CallFunction|GetGM))))

(event Input|MouseEvents|LeftMouseButton
  (params (Key :type Key%20Structure))
  (bind _gm (CallFunction|GetGM))
  (:Pressed
    (switch Utilities|FlowControl|Switch|SwitchonE_GamePhase (Variables|/Game/Grotoro/Gameplay/BP_GameMode.BP_GameMode_C|GetPhase _gm)
      (:NewEnumerator0
        _)
      (:NewEnumerator4
        _))
    (Default|Next _gm)))

(fn ConstructionScript)