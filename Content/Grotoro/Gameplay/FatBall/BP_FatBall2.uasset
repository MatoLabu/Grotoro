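; BP_FatBall2 is a musical ball that flies in a random horizontal direction, bouncing off walls, other fat balls and the pawn.
; Wall bounces copy relative transforms between the wall's two direction helpers to redirect the ball, and arm its sound.
; The sound manager's next beat plays the randomized sound and spawns a tempo-timed impact at the bounce point.
; Construction slightly randomizes both membrane colors, which the impact inherits.
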(event OnComponentBeginOverlap(Collision_StickWall)
  (params (OverlappedComponent :type Primitive%20Component%20Object%20Reference) (OtherActor :type Actor%20Object%20Reference) (OtherComp :type Primitive%20Component%20Object%20Reference) (OtherBodyIndex :type Integer) (bFromSweep :type Boolean) (SweepResult :type Hit%20Result%20Structure%20%28by%20ref%29))
  (bind _direction (Variables|Default|GetDirection))
  (bind _returnvalue (Transformation|GetWorldTransform _direction))
  ;[1 1 1] Collide with wall
  (bind _asbp_wall_collision (Utilities|Casting|CastToBP_WallCollision OtherActor)
    (:then
      (Variables|Default|SetCollidedWall _asbp_wall_collision)
      (Transformation|SetWorldLocationAndRotation (Variables|/Game/Grotoro/Gameplay/LevelDesign/BP_WallCollision.BP_WallCollision_C|GetFBDirection (Variables|Default|GetCollidedWall)) (.location _returnvalue) (.rotation _returnvalue) false false)
      (Transformation|SetRelativeLocationAndRotation (Variables|/Game/Grotoro/Gameplay/LevelDesign/BP_WallCollision.BP_WallCollision_C|GetBounceFBDirection (Variables|Default|GetCollidedWall)) (.location (Transformation|GetRelativeTransform (Variables|/Game/Grotoro/Gameplay/LevelDesign/BP_WallCollision.BP_WallCollision_C|GetFBDirection (Variables|Default|GetCollidedWall)))) (.rotation (Transformation|GetRelativeTransform (Variables|/Game/Grotoro/Gameplay/LevelDesign/BP_WallCollision.BP_WallCollision_C|GetFBDirection (Variables|Default|GetCollidedWall)))) false false)
      (Transformation|SetWorldLocationAndRotation (Variables|Default|GetDirection) (.location (Transformation|GetWorldTransform (Variables|/Game/Grotoro/Gameplay/LevelDesign/BP_WallCollision.BP_WallCollision_C|GetBounceFBDirection (Variables|Default|GetCollidedWall)))) (.rotation (Transformation|GetWorldTransform (Variables|/Game/Grotoro/Gameplay/LevelDesign/BP_WallCollision.BP_WallCollision_C|GetBounceFBDirection (Variables|Default|GetCollidedWall)))) false false)
      (Variables|Default|SetInitLocation (Transformation|GetActorLocation))
      (Variables|Default|SetbActivateSound true) ; B to let sound be triggered
    )
    (:CastFailed
      (bind _asbp_fat_ball_2 (Utilities|Casting|CastToBP_FatBall2 OtherActor)
        (:then
          (Transformation|SetWorldRotation (Variables|Default|GetDirection) (Math|Rotator|MakeRotator 0.0 0.0 (.yaw (Math|Rotator|FindLookatRotation (Transformation|GetActorLocation _asbp_fat_ball_2) (Transformation|GetActorLocation)))) false false))
        (:CastFailed
          (bind _asbp_pawn (Utilities|Casting|CastToBP_Pawn OtherActor))
          (Transformation|SetWorldRotation (Variables|Default|GetDirection) (Math|Rotator|MakeRotator 0.0 0.0 (.yaw (Math|Rotator|FindLookatRotation (Transformation|GetActorLocation _asbp_pawn) (Transformation|GetActorLocation)))) false false))))))

(event Custom|EjectPlayer
  (bind _collision_ejectplayer (Variables|Default|GetCollision_EjectPlayer))
  ;[1 0 0] OLD
  ;;[1 1 1] Eject player after glue
  (Collision|SetCollisionResponsetoAllChannels _collision_ejectplayer "ECR_Block")
  (Utilities|FlowControl|Delay 0.01)
  (Collision|SetCollisionResponsetoAllChannels _collision_ejectplayer "ECR_Overlap"))

(event Custom|Trigger%20Impact
  (bind _returnvalue (Math|Random|RandomIntegerinRange 0 1))
  (Game|SpawnActorfromClass "/Game/Grotoro/Art/Impacts/BP_WallImpacts.BP_WallImpacts_C" (Math|Transform|MakeTransform (Variables|Default|GetInitLocation) "0, 0, 0" "1,1,1") "Undefined" 0 (Variables|Default|GetCamaieuMain) (Variables|Default|GetCamaieuSecond) (/ (Utilities|Select :Index (Variables|/Game/Grotoro/Sound/Bp_SoundManager.Bp_SoundManager_C|GetMusicBpm (Variables|Default|GetBpSoundManager)) :NewEnumerator0 (Utilities|Select :Index _returnvalue :Option%200 1.0 :Option%201 2.0) :NewEnumerator1 (Utilities|Select :Index _returnvalue :Option%200 0.857 :Option%201 1.714) :NewEnumerator2 (Utilities|Select :Index _returnvalue :Option%200 0.75 :Option%201 1.5)) 2.0) 7.0 0 :!pinned true) ; Spawn Impact Sphere
)

(event Custom|Beat
  (CallFunction|TriggerSound))

(event Custom|TriggerSound
  (bind _a_ballsound (Variables|Default|GetA_BallSound))
  ;[1 1 1] Musical Balls
  (if (Variables|Default|GetbActivateSound)
    (Variables|Default|SetA_SoundTypeParameter (Math|Conversions|ToFloat(Integer) (Math|Random|RandomIntegerinRange 0 9)))
    (Class|FMODAudioComponent|SetParameter _a_ballsound "TriggerBells" (Variables|/Game/Grotoro/Sound/Bp_SoundManager.Bp_SoundManager_C|GetRootNoteIndex (Variables|Default|GetBpSoundManager)))
    (Class|FMODAudioComponent|SetParameter _a_ballsound "BallsType" (Variables|Default|GetA_SoundTypeParameter))
    (if (Math|Random|RandomBoolwithWeight 0.6)
      (Class|FMODAudioComponent|SetParameter _a_ballsound "BallPitch" 0.0)
      (else
        (Class|FMODAudioComponent|SetParameter _a_ballsound "BallPitch" (Math|Conversions|ToFloat(Integer) (Math|Random|RandomIntegerinRange 1 2)))))
    (Class|FMODAudioComponent|Play _a_ballsound)
    (CallFunction|TriggerImpact)
    (Variables|Default|SetbActivateSound false)))

(event EventBeginPlay
  ;[1 1 1] random direction
  (Transformation|SetWorldRotation (Variables|Default|GetDirection) (Math|Rotator|MakeRotator 0.0 0.0 (Math|Random|RandomFloatinRange 0.0 3.6e+02)) false false)
  (bind _outactors (Actor|GetAllActorsOfClass "/Game/Grotoro/Sound/Bp_SoundManager.Bp_SoundManager_C"))
  (Variables|Default|SetBpSoundManager (Utilities|Array|Get(acopy) _outactors))
  (EventDispatchers|BindEventtoTriggerBeat (Variables|Default|GetBpSoundManager) (delegate Custom|Beat)))

(event EventTick
  (params (DeltaSeconds :type Float%20%28single-precision%29))
  ;[1 1 1] fly in air
  (if (not (Variables|Default|GetIsStuck))
    (Transformation|AddActorWorldOffset (* (Math|Vector|GetForwardVector (Variables|Default|GetDirection)) (* (Variables|Default|GetEjectionSpeed) (Utilities|Time|GetWorldDeltaSeconds) 1e+02)))))

(fn ConstructionScript
  (bind _maincolor (Variables|Default|GetMainColor))
  (bind _secondcolor (Variables|Default|GetSecondColor))
  (bind _returnvalue (Rendering|Material|CreateDynamicMaterialInstance (Variables|Default|GetFatBall) 0 "/Game/Grotoro/Art/Character/Heart/M_Membrane_Inst.M_Membrane_Inst" :!class /Script/Engine.PrimitiveComponent))
  (bind _output_get (Variables|Default|SetCamaieuMain (Utilities|Struct|MakeLinearColor (+ (.r _maincolor) (Math|Random|RandomFloatinRange 0.02 -0.02)) (+ (Math|Random|RandomFloatinRange 0.07 -0.07) (.g _maincolor)) (+ (Math|Random|RandomFloatinRange 0.07 -0.07) (.b _maincolor)) 1.0)))
  (Rendering|Material|SetVectorParameterValue _returnvalue "MainColor" _output_get :!class /Script/Engine.MaterialInstanceDynamic)
  (bind _output_get_2 (Variables|Default|SetCamaieuSecond (Utilities|Struct|MakeLinearColor (+ (.r _secondcolor) (Math|Random|RandomFloatinRange 0.02 -0.02)) (+ (.g _secondcolor) (Math|Random|RandomFloatinRange 0.07 -0.07)) (+ (.b _secondcolor) (Math|Random|RandomFloatinRange 0.07 -0.07)) 1.0)))
  (Rendering|Material|SetVectorParameterValue _returnvalue "SecondColor" _output_get_2 :!class /Script/Engine.MaterialInstanceDynamic))