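; BP_FatBall is a projectile that flies in a random horizontal direction until it sticks to a wall and becomes a glue surface.
; Tick moves it unswept along the Direction component until it overlaps a component tagged "wall".
; On sticking, it blocks all channels, swaps to the bouncing material and tags its glue collision.
; EjectPlayer briefly toggles another collision from Block back to Overlap to eject a glued player.
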(event OnComponentBeginOverlap(Collision_StickWall)
  (params (OverlappedComponent :type Primitive%20Component%20Object%20Reference) (OtherActor :type Actor%20Object%20Reference) (OtherComp :type Primitive%20Component%20Object%20Reference) (OtherBodyIndex :type Integer) (bFromSweep :type Boolean) (SweepResult :type Hit%20Result%20Structure%20%28by%20ref%29))
  ;[1 1 1] Collide with wall
  ;[1 1 1] Set stuck in the wall
  (if (Components|ComponentHasTag OtherComp "wall")
    (Variables|Default|SetIsStuck true)
    ;[1 1 1] Block all
    (Collision|SetCollisionResponsetoAllChannels (Variables|Default|GetCollision_StickWall) "ECR_Block")
    ;[1 1 1] Change color
    (Rendering|Material|SetMaterial (Variables|Default|GetFatBall) 0 "/Game/Grotoro/Art/Blobs/M_Bouncing_Inst.M_Bouncing_Inst")
    (Variables|/Script/Engine.ActorComponent|SetComponentTags (Variables|Default|GetCollision_Glue) (Utilities|Array|MakeArray "glue"))))

(event Custom|EjectPlayer
  (bind _collision_ejectplayer (Variables|Default|GetCollision_EjectPlayer))
  ;[1 1 1] Eject player after glue
  (Collision|SetCollisionResponsetoAllChannels _collision_ejectplayer "ECR_Block")
  (Utilities|FlowControl|Delay 0.01)
  (Collision|SetCollisionResponsetoAllChannels _collision_ejectplayer "ECR_Overlap"))

(event EventBeginPlay
  ;[1 1 1] random direction
  (Transformation|SetWorldRotation (Variables|Default|GetDirection) (Math|Rotator|MakeRotator 0.0 0.0 (Math|Random|RandomFloatinRange 0.0 3.6e+02)) false false))

(event EventTick
  (params (DeltaSeconds :type Float%20%28single-precision%29))
  ;[1 1 1] fly in air
  (if (not (Variables|Default|GetIsStuck))
    (Transformation|AddActorWorldOffset (* (Math|Vector|GetForwardVector (Variables|Default|GetDirection)) (* (Variables|Default|GetEjectionSpeed) (Utilities|Time|GetWorldDeltaSeconds) 1e+02)))))

(fn ConstructionScript)