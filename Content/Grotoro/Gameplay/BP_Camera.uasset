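; BP_Camera is the gameplay camera Blueprint for Grotoro, acting as a central trigger for camera shakes.
; Each custom event covers a feedback moment such as dashes, dash clashes, hits, Ole jumps and falls, or death.
; Every event plays its own shake class as a world shake at the Camera component's location, using a small outer radius so it affects only views at that spot.
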(event Custom|ShakeGrotoro
  (Camera|PlayWorldCameraShake "/Game/Grotoro/Art/ShakeCam/CS_Grotoro.CS_Grotoro_C" (Transformation|GetWorldLocation (Variables|Default|GetCamera)) 0.0 1e+01))

(event Custom|CS_DashVsDash
  (Camera|PlayWorldCameraShake "/Game/Grotoro/Art/ShakeCam/CS_DashVsDash.CS_DashVsDash_C" (Transformation|GetWorldLocation (Variables|Default|GetCamera)) 0.0 1e+01))

(event Custom|CS_OleJump
  (Camera|PlayWorldCameraShake "/Game/Grotoro/Art/ShakeCam/CS_OleJump.CS_OleJump_C" (Transformation|GetWorldLocation (Variables|Default|GetCamera)) 0.0 1e+01))

(event Custom|CS_OleFall
  (Camera|PlayWorldCameraShake "/Game/Grotoro/Art/ShakeCam/CS_OleFall.CS_OleFall_C" (Transformation|GetWorldLocation (Variables|Default|GetCamera)) 0.0 1e+01))

(event Custom|CS_Dash
  (Camera|PlayWorldCameraShake "/Game/Grotoro/Art/ShakeCam/CS_Dash.CS_Dash_C" (Transformation|GetWorldLocation (Variables|Default|GetCamera)) 0.0 1e+01))

(event Custom|CS_1PV
  (Camera|PlayWorldCameraShake "/Game/Grotoro/Art/ShakeCam/CS_1PV.CS_1PV_C" (Transformation|GetWorldLocation (Variables|Default|GetCamera)) 0.0 1e+01))

(event Custom|CS_Death
  (Camera|PlayWorldCameraShake "/Game/Grotoro/Art/ShakeCam/CS_Death.CS_Death_C" (Transformation|GetWorldLocation (Variables|Default|GetCamera)) 0.0 1e+01))

(event Custom|CS_DashInWall
  (Camera|PlayWorldCameraShake "/Game/Grotoro/Art/ShakeCam/CS_DashInWall.CS_DashInWall_C" (Transformation|GetWorldLocation (Variables|Default|GetCamera)) 0.0 1e+01))

(event Custom|ShakeGro
  (Camera|PlayWorldCameraShake "/Game/Grotoro/Art/ShakeCam/CS_Gro.CS_Gro_C" (Transformation|GetWorldLocation (Variables|Default|GetCamera)) 0.0 1e+01))

(event Custom|CS_Hit
  (Camera|PlayWorldCameraShake "/Game/Grotoro/Art/ShakeCam/CS_Hit.CS_Hit_C" (Transformation|GetWorldLocation (Variables|Default|GetCamera)) 0.0 1e+01))

(fn ConstructionScript)