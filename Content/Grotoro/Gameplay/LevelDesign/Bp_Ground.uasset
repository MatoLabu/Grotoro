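; Ground level-design actor whose star and cloud particle effects can be launched and deactivated.
; Launching starts a randomly delayed timer that plays a Rotation timeline at a random rate, lerping both effects toward a small random pitch and roll or yaw offset in world rotation.
; Each finished turn stores its target as the next start rotation and re-arms the timer, producing continuous irregular drift.
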(event Custom|Deactivate%20Particles
  (Components|Activation|Deactivate (Variables|Default|GetP_Stars)))

(event Custom|MakeStarsRot
  (Components|Timeline|SetPlayRate (Variables|Default|GetRotation) (Math|Random|RandomFloatinRange 0.1 1.0))
  (Variables|Default|SetTargetRot (Math|Rotator|MakeRotator (Math|Random|RandomFloatinRange -1e+01 1e+01) (Math|Random|RandomFloatinRange -1e+01 1e+01) (Math|Random|RandomFloatinRange 0.0 0.0)))
  (bind _alpha (Timeline|Rotation PlayFromStart)
    (:Update
      (Transformation|SetWorldRotation (Variables|Default|GetP_Clouds) (Math|Rotator|Lerp(Rotator) (Variables|Default|GetSphereRot) (Variables|Default|GetTargetRot) _alpha) false false))
    (:Finished
      (Variables|Default|SetSphereRot (Variables|Default|GetTargetRot))
      (CallFunction|SetTimerRot))))

(event Custom|LaunchParticles
  (Components|Activation|Activate (Variables|Default|GetP_Stars) false)
  (CallFunction|SetTimerRot))

(event Custom|SetTimerRot
  (Utilities|Time|SetTimerbyEvent (delegate Custom|MakeStarsRot) (Math|Random|RandomFloatinRange 4.0 1e+01)))

(event EventBeginPlay)

(fn ConstructionScript)

(fn RandomVelocity
  (params (MinX :type Float%20%28single-precision%29) (MaxX :type Float%20%28single-precision%29) (MinY :type Float%20%28single-precision%29) (MaxY :type Float%20%28single-precision%29) (MinZ :type Float%20%28single-precision%29) (MaxZ :type Float%20%28single-precision%29))
  (return (Math|Random|RandomFloatinRange MinX MaxX) (Math|Random|RandomFloatinRange MinY MaxY) (Math|Random|RandomFloatinRange MinZ MaxZ)))