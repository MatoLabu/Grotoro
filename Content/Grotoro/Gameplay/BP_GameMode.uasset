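; Game mode for a local multiplayer game, running phases from title, how-to-play and countdown through play to game over and level restart.
; On BeginPlay it applies low scalability settings, lowering screen percentage if FPS stays under 55, then spawns and possesses a pawn per player at tagged PlayerStarts.
; Phase events drive title, UI, ground particles and music through cached references.
; It also provides a brief time-dilation "Vlambeer sleep" hit-stop.
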(event Custom|PhaseHowToPlay
  ;[1 1 1] Phase HowToPlay
  (Variables|BP_GameMode_C|SetPhase (CallFunction|GetGM) "NewEnumerator1")
  (Default|MoveUp (Variables|Default|GetBPTitleRef))
  (Default|LoadInstruction (Variables|Default|GetUITitleScreenRef))
  (Default|LaunchParticles (Variables|Default|GetBP_Ground))
  (Utilities|FlowControl|Delay 0.3)
  (Variables|Default|SetCanSkipHowToPlay true))

(event Custom|PhaseGame
  ;[1 1 1] Phase Game
  (Variables|BP_GameMode_C|SetPhase (CallFunction|GetGM) "NewEnumerator3")
  (Default|MusicState (Variables|Default|GetBp_SoundManager) 2.0 0.0))

(event Custom|ResetDelayRestarGame
  ;[1 0 0] old
  (Timeline|DelayBeforeRestartGame PlayFromStart
    (:Finished
      (Development|ExecuteConsoleCommand "restartlevel"))))

(event Custom|AnyKeyActions
  (bind _a_bouncesound (Variables|Default|GetA_BounceSound))
  (bind _phase (Variables|Default|GetPhase))
  ;[1 1 1] Any Key actions
  ;[1 1 1] Bounce title letters
  (if (and (Variables|Default|GetGameIsReady) (or (Utilities|Enum|Equal(Enum) _phase "NewEnumerator0") (Utilities|Enum|Equal(Enum) _phase "NewEnumerator1")))
    (bind _outactors (Actor|GetAllActorsOfClass "/Game/Grotoro/Art/Title/BP_Letter.BP_Letter_C"))
    (for _array_element _outactors
      (if (not (Variables|/Game/Grotoro/Art/Title/BP_Letter.BP_Letter_C|GetIsBull _array_element))
        (Default|Bounce _array_element)))
    (Class|FMODAudioComponent|SetParameter _a_bouncesound "BallsType" (Math|Conversions|ToFloat(Integer) (Math|Random|RandomIntegerinRange 0 3)))
    (Class|FMODAudioComponent|Play _a_bouncesound)))

(event Custom|PhaseTitle
  ;[1 1 1] Phase Title
  (Variables|BP_GameMode_C|SetPhase (CallFunction|GetGM) "NewEnumerator0")
  (Default|BacktoCenter (Variables|Default|GetBPTitleRef))
  (Default|HideInstructions (Variables|Default|GetUITitleScreenRef))
  (Default|MusicState (Variables|Default|GetBp_SoundManager) 1.0 0.0))

(event Custom|PhaseGameOver
  (params (WinnerID :type Integer))
  ;[1 1 1] Phase GameOver
  (Variables|BP_GameMode_C|SetPhase (CallFunction|GetGM) "NewEnumerator4")
  ;[1 1 1] Music
  (Default|MusicState (Variables|Default|GetBp_SoundManager) 2.0 1.0)
  ;[1 1 1] PS
  (Default|DeactivateParticles (Variables|Default|GetBP_Ground))
  (Utilities|FlowControl|Delay 1.0)
  ;[1 1 1] UI
  (bind _returnvalue (UserInterface|CreateWidget "/Game/Grotoro/UI/UI_GameOver.UI_GameOver_C"))
  (Default|WIN _returnvalue WinnerID)
  (UserInterface|Viewport|AddtoViewport _returnvalue 0)
  ;[1 1 1] sfx
  (bind _returnvalue_2 (Class|FMODBlueprintStatics|PlayEvent2D "/Game/FMOD/Events/SFx/A_Victory.A_Victory" false))
  (Class|FMODBlueprintStatics|EventInstanceSetParameter _returnvalue_2 "PlayerN" (Math|Conversions|ToFloat(Integer) (- WinnerID 1)))
  (Class|FMODBlueprintStatics|EventInstancePlay _returnvalue_2)
  (Utilities|FlowControl|Delay 1.0)
  (Variables|Default|SetCanRestart true))

(event Custom|VlambeerSleep
  (params (MoreDelay :type Float%20%28single-precision%29))
  (Utilities|Time|SetGlobalTimeDilation 0.1)
  (Utilities|FlowControl|Delay (+ 0.015 MoreDelay))
  (Utilities|Time|SetGlobalTimeDilation 1.0))

(event Custom|PhaseCounter
  ;[1 1 1] Phase Counter
  (Utilities|FlowControl|Sequence
    (:then_1
      (Variables|BP_GameMode_C|SetPhase (CallFunction|GetGM) "NewEnumerator2")
      (Default|Counter (Variables|Default|GetBPTitleRef))
      (Rendering|SetActorHiddenInGame (Variables|Default|GetPlayers) false)
      (Default|HideMainMenu (Variables|Default|GetUITitleScreenRef)))))

(event Custom|Next
  ;[1 1 1] Action Next
  (switch Utilities|FlowControl|Switch|SwitchonE_GamePhase (Variables|Default|GetPhase)
    (:NewEnumerator0
      (CallFunction|PhaseHowtoPlay))
    (:NewEnumerator1
      (CallFunction|PhaseCounter))
    (:NewEnumerator4
      (if (Variables|Default|GetCanRestart)
        (Development|ExecuteConsoleCommand "restartlevel")))))

(event Custom|BounceTitleSound
  (bind _a_bouncesound (Variables|Default|GetA_BounceSound))
  ;[1 1 1] Bounce title letters
  (Class|FMODAudioComponent|SetParameter _a_bouncesound "BallsType" (Math|Conversions|ToFloat(Integer) (Math|Random|RandomIntegerinRange 0 3)))
  (Class|FMODAudioComponent|Play _a_bouncesound))

(event Custom|ActionQuit
  ;[1 1 1] ActionQuit
  (switch Utilities|FlowControl|Switch|SwitchonE_GamePhase (Variables|Default|GetPhase)
    (:NewEnumerator0
      (Development|ExecuteConsoleCommand "EXIT"))
    (:NewEnumerator1
      (Development|ExecuteConsoleCommand "restartlevel" :!label _label))
    (:NewEnumerator2
      (goto _label))
    (:NewEnumerator3
      (goto _label))
    (:NewEnumerator4
      (goto _label))))

(event EventBeginPlay
  ;[0.1467 1 0] BEGIN PLAY
  (bind _outactors (Actor|GetAllActorsOfClass "/Script/Engine.PlayerController"))
  (for _array_element _outactors
    (CallFunction|LogErer (Utilities|String|Append "At start, there is this playercontroller: " (Utilities|GetDisplayName _array_element))))
  (Utilities|FlowControl|Sequence
    (:then_0
      ;[1 1 1] Scalability Settings
      (CallFunction|SetRendering)
      (Utilities|FlowControl|Delay 1.0)
      (if (< (Variables|Default|GetFPS) 55.0)
        (Development|ExecuteConsoleCommand (Utilities|String|Append (Variables|Default|GetScreenPercentage) "75"))
        (Utilities|FlowControl|Delay 2.0)
        (if (< (Variables|Default|GetFPS) 55.0)
          (Development|ExecuteConsoleCommand (Utilities|String|Append (Variables|Default|GetScreenPercentage) "50"))))
      (Variables|Default|SetGameIsReady true)
      (Default|StartGame (Variables|Default|GetBPTitleRef))
      (Variables|Default|SetCanSkipTitle true)
      (CallFunction|GetPlayerStarts)
      (CallFunction|SpawnPlayers))
    (:then_1
      (Utilities|FlowControl|Delay 0.2)
      (CallFunction|MakeBPTitleREF)
      (CallFunction|MakeUITitleScreenREF))
    (:then_2
      ;[1 1 1] Set Listenner Position
      (bind _output_get (CallFunction|MakeBPSoundManagerREF))
      (Class|PlayerController|SetAudioListenerOverride (Game|GetPlayerController 0) (Variables|/Game/Grotoro/Sound/Bp_SoundManager.Bp_SoundManager_C|GetListener _output_get) "0, 0, 0" "0, 0, 0")
      (CallFunction|MakeBPGroundREF))))

(event EventTick
  (params (DeltaSeconds :type Float%20%28single-precision%29))
  ;[1 0.8415 0] EVENT TICK
  (Variables|Default|SetFPS (/ 1.0 DeltaSeconds)))

(fn ConstructionScript)

(fn MakeBPTitleREF
  (bind _outactors (Actor|GetAllActorsOfClass "/Game/Grotoro/Art/Title/BP_Title.BP_Title_C"))
  (Variables|Default|SetBPTitleRef (Utilities|Array|Get(acopy) _outactors)))

(fn MakeUITitleScreenREF
  (bind _foundwidgets (Widget|GetAllWidgetsOfClass "/Game/Grotoro/UI/UI_TitleScreen.UI_TitleScreen_C" true))
  (Variables|Default|SetUITitleScreenRef (Utilities|Array|Get(acopy) _foundwidgets)))

(fn MakeBPSoundManagerREF
  (bind _outactors (Actor|GetAllActorsOfClass "/Game/Grotoro/Sound/Bp_SoundManager.Bp_SoundManager_C"))
  (bind _output_get (Variables|Default|SetBp_SoundManager (Utilities|Array|Get(acopy) _outactors)))
  (return _output_get))

(fn MakeBPGroundREF
  (bind _outactors (Actor|GetAllActorsOfClass "/Game/Grotoro/Gameplay/LevelDesign/Bp_Ground.Bp_Ground_C"))
  (Variables|Default|SetBP_Ground (Utilities|Array|Get(acopy) _outactors)))

(fn GetCamera
  (bind _outactors (Actor|GetAllActorsOfClass "/Game/Grotoro/Gameplay/BP_Camera.BP_Camera_C"))
  (Game|Player|SetViewTargetwithBlend (Variables|Default|GetCurrentPlayerController) (Utilities|Array|Get(acopy) _outactors) 0.0 "VTBlend_Linear" 0.0 false))

(fn SetRendering
  (bind _asbp_game_instance (CallFunction|GetGI))
  (if (Variables|/Game/Grotoro/Gameplay/BP_GameInstance.BP_GameInstance_C|GetFirstStart _asbp_game_instance)
    (Development|ExecuteConsoleCommand "r.ScreenPercentage 100")
    (Variables|/Game/Grotoro/Gameplay/BP_GameInstance.BP_GameInstance_C|SetFirstStart _asbp_game_instance false))
  (Development|ExecuteConsoleCommand "r.vsynceditor 0")
  (Development|ExecuteConsoleCommand "r.vsync 0")
  (Development|ExecuteConsoleCommand "r.ViewDistanceScale 1")
  (Development|ExecuteConsoleCommand "r.PostProcessAAQuality 4")
  (Development|ExecuteConsoleCommand "sg.PostProcessQuality 0")
  (Development|ExecuteConsoleCommand "sg.ShadowQuality 0")
  (Development|ExecuteConsoleCommand "sg.TextureQuality 0")
  (Development|ExecuteConsoleCommand "sg.EffectsQuality 0")
  (Development|ExecuteConsoleCommand "r.DetailMode 0")
  (Development|ExecuteConsoleCommand "FoliageQuality 0"))

(fn GetPlayerStarts
  (bind _outactors (Actor|GetAllActorsOfClass "/Script/Engine.PlayerStart"))
  (Variables|Default|SetPlayerStartsREF _outactors))

(fn SpawnPlayers
  (for _index (range (LocalVariables|GetFirstIndex) (- (Variables|Default|GetPlayerCount) 1))
    (Variables|Default|SetIndex _index)
    (CallFunction|TaketheGoodPlayerStart)
    (CallFunction|CreatePlayerSlot)
    ;[1 1 1] spawn
    (bind _returnvalue (Game|SpawnActorfromClass "/Game/Grotoro/Gameplay/Character/BP_Pawn.BP_Pawn_C" (Transformation|GetActorTransform (Variables|Default|GetPlayerStart)) "AlwaysSpawn" (Variables|Default|GetCurrentPlayerController) (+ (Variables|Default|GetIndex) 1) 0))
    (Variables|Default|SetNewPawn _returnvalue)
    ;[1 1 1] associate to PCont
    (Pawn|Possess (Variables|Default|GetCurrentPlayerController) (Variables|Default|GetNewPawn))
    ;[1 1 1] Ref
    (Utilities|Array|AddUnique (Variables|Default|GetPlayers) (Variables|Default|GetNewPawn))
    (CallFunction|GetCamera))
  (Variables|/Game/Grotoro/Gameplay/BP_GameInstance.BP_GameInstance_C|SetPContNeedToBeCreated (CallFunction|GetGI) false))

(fn TaketheGoodPlayerStart
  (for _array_element (Variables|Default|GetPlayerStartsREF)
    (if (Utilities|Name|Equal(Name) (Variables|/Script/Engine.PlayerStart|GetPlayerStartTag _array_element) (Utilities|String|StringToName (Utilities|String|ToString(Integer) (Variables|Default|GetIndex))))
      (bind _output_get (Variables|Default|SetPlayerStart _array_element)))))

(fn CreatePlayerSlot
  (bind _playercontrollers (Variables|Default|GetPlayerControllers))
  (bind _index (Variables|Default|GetIndex))
  (if (Variables|/Game/Grotoro/Gameplay/BP_GameInstance.BP_GameInstance_C|GetPContNeedToBeCreated (CallFunction|GetGI))
    (if (== _index 0)
      (Variables|Default|SetCurrentPlayerController (Game|GetPlayerController 0))
      (else
        (bind _returnvalue (Class|GameplayStatics|CreatePlayer _index))
        (Variables|Default|SetCurrentPlayerController _returnvalue)))
    (else
      (Variables|Default|SetCurrentPlayerController (Game|GetPlayerController _index))))
  (Utilities|Array|AddUnique _playercontrollers (Variables|Default|GetCurrentPlayerController))
  (CallFunction|LogErer (Utilities|String|Append "Verification PCont: " (Utilities|GetDisplayName (Utilities|Array|Get(acopy) _playercontrollers _index)))))