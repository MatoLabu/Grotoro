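; Player controller that turns Player 1's input into facing rotation for the Player1 object.
; Axis events cache X and Y values, and Tick calls GetWantedRotation then Player1.Rotate whenever either is non-zero.
; GetWantedRotation sets P1WantedDirection only for exact cardinal inputs; diagonal checks are unwired.
; Older Move, Turn and logging paths are disconnected, and the Up and Right actions drive no movement here.
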(event EventTick
  (params (DeltaSeconds :type Float%20%28single-precision%29))
  (if (or (!= (Variables|Default|GetP1YValue) 0.0) (!= (Variables|Default|GetP1XValue) 0.0))
    (CallFunction|GetWantedRotation)
    (Default|Rotate (Variables|Default|GetPlayer1))))

(event Input|ActionEvents|InputActionP1Up
  (params (Key :type Key%20Structure))
  (:Pressed
    (Variables|Default|SetP1Up true))
  (:Released
    (Variables|Default|SetP1Up false)))

(event Input|ActionEvents|InputActionP1Right
  (params (Key :type Key%20Structure))
  (:Pressed
    (Utilities|IfPlayerValid (Variables|Default|GetPlayer1))))

(event Input|AxisEvents|InputAxisP1Turn
  (params (AxisValue :type Float%20%28single-precision%29))
  (Variables|Default|SetP1XValue AxisValue))

(event Input|AxisEvents|InputAxisP1MoveY
  (params (AxisValue :type Float%20%28single-precision%29))
  (Variables|Default|SetP1YValue AxisValue))

(fn ConstructionScript)

(fn GetWantedRotation
  (if (and (== (Variables|Default|GetP1YValue) 1.0) (== (Variables|Default|GetP1XValue) 0.0))
    (Variables|Default|SetP1WantedDirection "0,0.000000,0.000000")
    (elif (and (== (Variables|Default|GetP1YValue) -1.0) (== (Variables|Default|GetP1XValue) 0.0))
      (Variables|Default|SetP1WantedDirection "0,180.000000, 0")
      (elif (and (== (Variables|Default|GetP1YValue) 0.0) (== (Variables|Default|GetP1XValue) 1.0))
        (Variables|Default|SetP1WantedDirection "0,90.000000, 0")
        (elif (and (== (Variables|Default|GetP1YValue) 0.0) (== (Variables|Default|GetP1XValue) -1.0))
          (Variables|Default|SetP1WantedDirection "0,270.000000, 0"))))))